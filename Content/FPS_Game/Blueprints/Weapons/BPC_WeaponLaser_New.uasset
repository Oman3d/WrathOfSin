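; Laser weapon Blueprint that extends a parent weapon class with an ammo readout on a TextRender component.
; It calls the parent's begin play, fire and reload logic, refreshing the displayed current ammo count after BeginPlay, WeaponFire and Reload.
; Every tick, it shows the text only while the cached player is in first-person view.
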(event `self.ReceiveTick`
  (params (DeltaSeconds :type "Float (single-precision)"))
  (bind _playercast (`self.PlayerCast`))
  (`/Engine/EditorBlueprintResources/StandardMacros.IsValid` _playercast
    (:`Is Valid`
      (`SceneComponent.SetVisibility` (`self.TextRender`) (`/Game/MainLevels/Player/BP_CharacterBase.isFPP` _playercast) false))))

(event `self.ReceiveBeginPlay`
  (`parent.ReceiveBeginPlay`)
  (`TextRenderComponent.K2_SetText` (`self.TextRender`) (`KismetTextLibrary.Conv_IntToText` (`self.AmmoCurrent`)) :!label _label))

(event `self.WeaponFire`
  (`parent.WeaponFire`)
  (goto _label))

(event `self.ReloadWeapon`
  (`parent.ReloadWeapon`))

(event `self.Reload`
  (`parent.Reload`)
  (goto _label))

(fn `UserConstructionScript`
  (`parent.UserConstructionScript`))