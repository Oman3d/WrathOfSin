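; BP_QuestGiver is an example quest-giver character that wanders the navmesh and hands out quests when a player interacts with it.
; It loops AI moves to random points around its start location, pausing between moves.
; Player overlap with the quest target component stops movement and holds the loop until the overlap ends.
; Interaction first tries to finish an "Interaction" objective, otherwise asks the player's quest manager to take a quest.
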(event `self.ReceiveBeginPlay`
  (set `self.StartLoc` (`self.K2_GetActorLocation`))
  (bind _randomlocation (`NavigationSystemV1.K2_GetRandomLocationInNavigableRadius` (`self.StartLoc`) 1500.0 null null :!label _label))
  (`|AIMoveTo` self _randomlocation null
    (:`OnSuccess`
      _)
    (:`OnFail`
      _))
  (`KismetSystemLibrary.Delay` 2.0)
  (if (`self.IsInterrupted`) :!label _label_2
    (`KismetSystemLibrary.Delay` 0.2)
    (goto _label_2)
    (else
      (goto _label))))

(event `self.Manager_QuestTarget.On_QuestTarget_Interacted`
  (params (OverlappedBoxTag :type Name) (ByPawn :type "Pawn Object Reference"))
  (bind _success (`/Game/QuestManager/Blueprints/Components/Manager_QuestTarget.Try_Finish_Objective` (`self.Manager_QuestTarget`) "Interaction" ByPawn))
  (if (not _success)
    (bind _returnvalue (`/Game/QuestManager/Blueprints/Data/Libraries/ML_MissionComponent.Get_Quest_Manager` (`self.GetController` ByPawn))
      (:`then`
        (`/Game/QuestManager/Blueprints/Components/Manager_Mission.Try_Take_Quest` _returnvalue)))))

(event `self.Manager_QuestTarget.On_QuestTarget_Begin_Overlap`
  (params (ByPawn :type "Pawn Object Reference") (OverlappedBoxTag :type Name))
  (set `self.IsInterrupted` true)
  (`MovementComponent.StopMovementImmediately` (`self.CharacterMovement`)))

(event `self.Manager_QuestTarget.On_QuestTarget_End_Overlap`
  (params (ByPawn :type "Pawn Object Reference") (OverlappedBoxTag :type Name))
  (set `self.IsInterrupted` false))

(fn `UserConstructionScript`
  (`/Game/QuestManager/Blueprints/Components/Manager_QuestTarget.Construct_InteractionBox` (`self.Manager_QuestTarget`)))