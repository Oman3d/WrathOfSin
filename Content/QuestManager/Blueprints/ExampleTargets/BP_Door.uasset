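; BP_Door is an example quest target: a sliding door that opens when a player interacts with it.
; Its Manager_QuestTarget component builds the interaction box at construction and reports interactions.
; An interaction on a closed, idle door starts the toggle, tries to finish the "Interaction" objective and disables the handle.
; The DoorToggle timeline is set up to lerp the Cube's relative Y between closed and open offsets, flipping DoorIsOpened when finished.
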(event `Start_Toggle_Door`
  (set `self.StartDeltaY` (`KismetMathLibrary.SelectFloat` -400.0 0.0 (`self.DoorIsOpened`)))
  (set `self.TargetDeltaY` (`KismetMathLibrary.SelectFloat` 0.0 -400.0 (`self.DoorIsOpened`)))
  (`TimelineComponent.PlayFromStart` (`self.Door Toggle`)))

(event `self.Manager_QuestTarget.On_QuestTarget_Interacted`
  (params (OverlappedBoxTag :type Name) (ByPawn :type "Pawn Object Reference"))
  (if (and (not (`self.DoorIsOpened`)) (not (`TimelineComponent.IsPlaying` (`self.Door Toggle`))))
    (`self.Start_Toggle_Door`)
    (`/Game/QuestManager/Blueprints/Components/Manager_QuestTarget.Try_Finish_Objective` (`self.Manager_QuestTarget`) "Interaction" ByPawn)
    (`/Game/QuestManager/Blueprints/Components/Manager_QuestTarget.Set_Interaction_Enabled` (`self.Manager_QuestTarget`) "DoorHandle" false)))

(fn `UserConstructionScript`
  (set `/Game/QuestManager/Blueprints/Components/Manager_QuestTarget.TargetName` (`self.TargetName`) (`self.Manager_QuestTarget`))
  (`/Game/QuestManager/Blueprints/Components/Manager_QuestTarget.Construct_InteractionBox` (`self.Manager_QuestTarget`)))