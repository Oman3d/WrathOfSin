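; Example quest giver actor that offers a quest to the player on overlap through the Quest Manager.
; Overlaps from its quest target component or its Box (characters only) fetch the relevant controller's quest manager and call TryTakeQuest.
; The construction script builds the component's interaction box.
; The interaction event is empty, and the logic to try finishing an "Interaction" objective first is disconnected.
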(event `self.Manager_QuestTarget.On_QuestTarget_Interacted`
  (params (OverlappedBoxTag :type Name) (ByPawn :type "Pawn Object Reference")))

(event `self.Manager_QuestTarget.On_QuestTarget_Begin_Overlap`
  (params (ByPawn :type "Pawn Object Reference") (OverlappedBoxTag :type Name))
  (bind _returnvalue (`/Game/QuestManager/Blueprints/Data/Libraries/ML_MissionComponent.Get_Quest_Manager` (`Pawn.GetController` ByPawn))
    (:`then`
      (`/Game/QuestManager/Blueprints/Components/Manager_Mission.Try_Take_Quest` _returnvalue))))

(event `self.Box.OnComponentBeginOverlap`
  (params (OverlappedComponent :type "PrimitiveComponent Object Reference") (OtherActor :type "Actor Object Reference") (OtherComp :type "PrimitiveComponent Object Reference") (OtherBodyIndex :type Integer) (bFromSweep :type Boolean) (SweepResult :type "HitResult Structure (by ref)"))
  (cast `/Game/MainLevels/Player/BP_CharacterBase` OtherActor)
  (bind _returnvalue (`/Game/QuestManager/Blueprints/Data/Libraries/ML_MissionComponent.Get_Quest_Manager` (`GameplayStatics.GetPlayerController` 0))
    (:`then`
      (`/Game/QuestManager/Blueprints/Components/Manager_Mission.Try_Take_Quest` _returnvalue))))

(fn `UserConstructionScript`
  (`/Game/QuestManager/Blueprints/Components/Manager_QuestTarget.Construct_InteractionBox` (`self.Manager_QuestTarget`)))