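; Example quest-giver actor that hands a named quest to the player through the quest manager, then locks and destroys itself.
; It registers as a quest giver on BeginPlay and assigns either on quest-target overlap, once a character has entered its Box, or via an Open/On call when CallToAssignQuest is set.
; Construction configures the box and labels per mode.
; Save hooks cache state and destroy an already-locked giver on restore.
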(event `self.Open/On`
  (params (HorrorEvent :type Boolean))
  (if (`self.Call to Assign Quest`)
    (`self.AddQuest`)
    (elif (`self.Turn On Collison`)
      (`PrimitiveComponent.SetCollisionEnabled` (`self.Box`) "QueryAndPhysics"))))

(event `self.ReceiveBeginPlay`
  (bind _asplayer_state_quest_manager (cast `/Game/QuestManager/Blueprints/Framework/PlayerState_QuestManager` (`GameplayStatics.GetPlayerState` 0)))
  (`KismetArrayLibrary.Array_Add` (`/Game/QuestManager/Blueprints/Components/Manager_Mission.Manuel Add to Quest Givers` (`/Game/QuestManager/Blueprints/Framework/PlayerState_QuestManager.Manager_Mission` _asplayer_state_quest_manager)) (make `/Game/QuestManager/Blueprints/Data/Structs/Struct_ActiveQuestGiver` (`self.Quest Target Name`) (`self.Unque Quest Name`)))
  (if (`self.Turn On Collison`)
    (`PrimitiveComponent.SetCollisionEnabled` (`self.Box`) "QueryAndPhysics")
    (else
      (`PrimitiveComponent.SetCollisionEnabled` (`self.Box`) "NoCollision"))))

(event `AddQuest`
  (if (`self.Open`)
    (bind _returnvalue (`/Game/QuestManager/Blueprints/Data/Libraries/ML_MissionComponent.Get_Quest_Manager` (`Pawn.GetController` (`self.By Pawn`)))
      (:`then`
        (`/Game/QuestManager/Blueprints/Components/Manager_Mission.Try_Take_Quest` _returnvalue)
        (set `self.Locked` true)
        (`self.K2_DestroyActor`)))))

(event `self.Manager_QuestTarget.On_QuestTarget_End_Overlap`
  (params (ByPawn :type "Pawn Object Reference") (OverlappedBoxTag :type Name)))

(event `self.Manager_QuestTarget.On_QuestTarget_Begin_Overlap`
  (params (ByPawn :type "Pawn Object Reference") (OverlappedBoxTag :type Name))
  (set `self.By Pawn` ByPawn)
  (if (not (`self.Call to Assign Quest`))
    (`self.AddQuest`)))

(event `self.Box.OnComponentBeginOverlap`
  (params (OverlappedComponent :type "PrimitiveComponent Object Reference") (OtherActor :type "Actor Object Reference") (OtherComp :type "PrimitiveComponent Object Reference") (OtherBodyIndex :type Integer) (bFromSweep :type Boolean) (SweepResult :type "HitResult Structure (by ref)"))
  (cast `/Game/MainLevels/Player/BP_CharacterBase` OtherActor)
  (set `self.Open` true))

(event `/Game/HorrorEngine/Blueprints/Core/HorrorEngineInterface.CollectSaveData`
  ;[1 1 1] Save Fuctions
  (bind _asmaster (`/Game/HorrorEngine/Blueprints/Core/HorrorEngineFunctions.GetPlayer`))
  (`KismetArrayLibrary.Array_Add` (`/Game/HorrorEngine/Blueprints/Core/HE_SaveGameComponent.AssetCache` (`/Game/HorrorEngine/HorrorEngine.HE_SaveGameComponent` _asmaster)) (make `/Game/HorrorEngine/Blueprints/Structures/SaveStructures/AssetsSave` (`KismetSystemLibrary.GetObjectName` self) (`self.Open`) (`self.Locked`) (`self.PlayerHasKey`) (`self.SliderLocked`) 0.0 0.0 0 "+00000000.00:00:00.000000000" "NewEnumerator0" (struct :`Actor` "NewEnumerator0" :`MeshSettings` (struct) :`InspectionSettings` (struct :`InspectionPivotLocation` (0.0 0.0 0.0) :`Takeable` true :`InspectionAnimation` true :`InspectionAnimationSpeedSec` 0.5 :`InspectionBeginRotation` (struct) :`InspectionBeginScale` 1.0 :`MinZoomScale` 1.0 :`MaxZoomScale` 2.0 :`RotationSpeed` 2.5 :`SlideSpeed` 1.0 :`MaxSlideValue` 10.0 :`ItemName` "NSLOCTEXT(\"[36B990E440B5BD7BCF070C96792ACD01]\", \"D9F7E24543A3C62D9A25D49182932C50\", \"Item Name\")" :`ItemInformation` "NSLOCTEXT(\"[36B990E440B5BD7BCF070C96792ACD01]\", \"D319F8FF45E02929BFE9029F7E4F92F2\", \"Item Information\")" :`ReadingText` "NSLOCTEXT(\"[36B990E440B5BD7BCF070C96792ACD01]\", \"7EC6767444499E5ADE0CC2AE6B98C1EB\", \"Reading Text\")" :`TakeButton` (struct :`ButtonText` "NSLOCTEXT(\"[36B990E440B5BD7BCF070C96792ACD01]\", \"035538DA4A617733A6BA3C9E56C8C353\", \"Take\")") :`ExamineButton` (struct :`ButtonText` "NSLOCTEXT(\"[36B990E440B5BD7BCF070C96792ACD01]\", \"98CD410B4C1C78FDE976DFAFA543FB6A\", \"Examine\")") :`ZoomSlideButton` (struct :`ButtonText` "NSLOCTEXT(\"[36B990E440B5BD7BCF070C96792ACD01]\", \"94E4F3C6409F91B925AAB29D107F0FAF\", \"Zoom/Slide\")") :`DismissButton` (struct :`ButtonText` "NSLOCTEXT(\"[36B990E440B5BD7BCF070C96792ACD01]\", \"534F19BF435BF6FA0D279D9CB68CE751\", \"Dismiss\")")) :`InventorySettings` (struct :`StorageType` "NewEnumerator3" :`NumberofItemstoAddInventory` 1 :`Interactable` true :`InteractionButton` (struct :`ButtonText` "NSLOCTEXT(\"[36B990E440B5BD7BCF070C96792ACD01]\", \"64A187E040DB8377D41CF0B31C6566EE\", \"Use\")") :`SwitchButton` (struct :`ButtonText` "NSLOCTEXT(\"[36B990E440B5BD7BCF070C96792ACD01]\", \"BAAFAC394A769DB19B68C7942605445D\", \"Switch\")") :`ZoomSlideButton` (struct :`ButtonText` "NSLOCTEXT(\"[36B990E440B5BD7BCF070C96792ACD01]\", \"1A097F0D4994134B413E229C769765DC\", \"Zoom/Slide\")") :`CloseInventoryButton` (struct :`ButtonText` "NSLOCTEXT(\"[36B990E440B5BD7BCF070C96792ACD01]\", \"0CE17A854283D46953A235BEC9899591\", \"Close\")")) :`Pistol_MeshSettingsTop` (struct) :`Vhs_CurrentTime` "+00000000.00:00:00.000000000"))))

(event `/Game/HorrorEngine/Blueprints/Core/HorrorEngineInterface.RestoreSaveData`
  (params (AssetSave :type "/Game/HorrorEngine/Blueprints/Structures/SaveStructures/AssetsSave Structure"))
  (bind ((`BooleanSlot01_63_ED79FB5D49E9ED6768D7AE96EDFDE8DB` _booleanslot01) (`BooleanSlot02_64_3DE3E28A45CAE9F3E913659977556562` _booleanslot02) (`BooleanSlot03_65_04AA048C42686C9D2AF003962AEB7F6C` _booleanslot03) (`BooleanSlot04_66_3CB4510F40F5DDD3D81BCEA77398809A` _booleanslot04)) (break `/Game/HorrorEngine/Blueprints/Structures/SaveStructures/AssetsSave` AssetSave))
  ;[1 1 1] Save Fuctions
  (set `self.Open` _booleanslot01)
  (set `self.Locked` _booleanslot02)
  (set `self.PlayerHasKey` _booleanslot03)
  (set `self.SliderLocked` _booleanslot04)
  (if (`self.Locked`)
    (`self.K2_DestroyActor`)))

(fn `UserConstructionScript`
  (`/Game/QuestManager/Blueprints/Components/Manager_QuestTarget.Construct_InteractionBox` (`self.Manager_QuestTarget`))
  (set `/Game/QuestManager/Blueprints/Components/Manager_QuestTarget.TargetName` (`self.Quest Target Name`) (`self.Manager_QuestTarget`))
  (`TextRenderComponent.K2_SetText` (`self.TextRender`) (`KismetTextLibrary.Conv_NameToText` (`self.Unque Quest Name`)))
  (if (`self.Call to Assign Quest`)
    (`BoxComponent.SetBoxExtent` (`self.Box`) (0.0 0.0 0.0) true)
    (set `self.Turn On Collison` false)
    (set `self.Open` true)
    (`TextRenderComponent.K2_SetText` (`self.TextRender1`) (`|FormatText` "Move close to Triggering Object "))
    (else
      (`BoxComponent.SetBoxExtent` (`self.Box`) (`self.In Box Extent`) true)
      (`TextRenderComponent.K2_SetText` (`self.TextRender1`) (`|FormatText` "Overlap Trigger")))))