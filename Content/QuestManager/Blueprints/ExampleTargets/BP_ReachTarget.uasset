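; Example quest target that completes a reach-location objective when an actor overlaps its box trigger.
; Overlap passes the ObjectiveTag and actor to ManagerQuestTarget.TryFinishObjective; on success the target sets Locked and destroys itself.
; The construction script sizes and raises the box from BoxExtent and names the quest target.
; Save events use the player's HESaveGameComponent asset cache, destroying the target on restore if Locked.
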(event `self.Box.OnComponentBeginOverlap`
  (params (OverlappedComponent :type "PrimitiveComponent Object Reference") (OtherActor :type "Actor Object Reference") (OtherComp :type "PrimitiveComponent Object Reference") (OtherBodyIndex :type Integer) (bFromSweep :type Boolean) (SweepResult :type "HitResult Structure (by ref)"))
  (bind _success (`/Game/QuestManager/Blueprints/Components/Manager_QuestTarget.Try_Finish_Objective` (`self.Manager_QuestTarget`) (`self.Objective Tag`) OtherActor))
  (if _success
    (set `self.Locked` true)
    (`self.K2_DestroyActor`)))

(event `/Game/HorrorEngine/Blueprints/Core/HorrorEngineInterface.CollectSaveData`
  ;[1 1 1] Save Fuctions
  (bind _asmaster (`/Game/HorrorEngine/Blueprints/Core/HorrorEngineFunctions.GetPlayer`))
  (`KismetArrayLibrary.Array_Add` (`/Game/HorrorEngine/Blueprints/Core/HE_SaveGameComponent.AssetCache` (`/Game/HorrorEngine/HorrorEngine.HE_SaveGameComponent` _asmaster)) (make `/Game/HorrorEngine/Blueprints/Structures/SaveStructures/AssetsSave` (`KismetSystemLibrary.GetObjectName` self) (`self.Open`) (`self.Locked`) (`self.PlayerHasKey`) (`self.SliderLocked`) 0.0 0.0 0 "+00000000.00:00:00.000000000" "NewEnumerator0" (struct :`Actor` "NewEnumerator0" :`MeshSettings` (struct) :`InspectionSettings` (struct :`InspectionPivotLocation` (0.0 0.0 0.0) :`Takeable` true :`InspectionAnimation` true :`InspectionAnimationSpeedSec` 0.5 :`InspectionBeginRotation` (struct) :`InspectionBeginScale` 1.0 :`MinZoomScale` 1.0 :`MaxZoomScale` 2.0 :`RotationSpeed` 2.5 :`SlideSpeed` 1.0 :`MaxSlideValue` 10.0 :`ItemName` "NSLOCTEXT(\"[0F87BF4C4CFDA5B6091A6E95288153C1]\", \"88E9A3B049D8C74A39D194BD0B48A7E7\", \"Item Name\")" :`ItemInformation` "NSLOCTEXT(\"[0F87BF4C4CFDA5B6091A6E95288153C1]\", \"94AC0A864585307E3A82179A85D26B04\", \"Item Information\")" :`ReadingText` "NSLOCTEXT(\"[0F87BF4C4CFDA5B6091A6E95288153C1]\", \"DF9F8991413DD4118DAFA7A369D852AA\", \"Reading Text\")" :`TakeButton` (struct :`ButtonText` "NSLOCTEXT(\"[0F87BF4C4CFDA5B6091A6E95288153C1]\", \"3F88B08F49E17441CFF8788F1CF71E88\", \"Take\")") :`ExamineButton` (struct :`ButtonText` "NSLOCTEXT(\"[0F87BF4C4CFDA5B6091A6E95288153C1]\", \"19A43764446577764056B0A80B94450B\", \"Examine\")") :`ZoomSlideButton` (struct :`ButtonText` "NSLOCTEXT(\"[0F87BF4C4CFDA5B6091A6E95288153C1]\", \"432CE1E846E032BB41412B9CEFBAE7E8\", \"Zoom/Slide\")") :`DismissButton` (struct :`ButtonText` "NSLOCTEXT(\"[0F87BF4C4CFDA5B6091A6E95288153C1]\", \"1D7A7B9A456790C4E4F3B9B1AC75B3BC\", \"Dismiss\")")) :`InventorySettings` (struct :`StorageType` "NewEnumerator3" :`NumberofItemstoAddInventory` 1 :`Interactable` true :`InteractionButton` (struct :`ButtonText` "NSLOCTEXT(\"[0F87BF4C4CFDA5B6091A6E95288153C1]\", \"ECA288AD44FC3FB5C4C3AD88F7C76447\", \"Use\")") :`SwitchButton` (struct :`ButtonText` "NSLOCTEXT(\"[0F87BF4C4CFDA5B6091A6E95288153C1]\", \"E5106FE94BE624F74901DAB424F55E9C\", \"Switch\")") :`ZoomSlideButton` (struct :`ButtonText` "NSLOCTEXT(\"[0F87BF4C4CFDA5B6091A6E95288153C1]\", \"8564E3B647A4B31279085ABFE0982F2F\", \"Zoom/Slide\")") :`CloseInventoryButton` (struct :`ButtonText` "NSLOCTEXT(\"[0F87BF4C4CFDA5B6091A6E95288153C1]\", \"FABC44BC4B4C2548066C978D8D084AA4\", \"Close\")")) :`Pistol_MeshSettingsTop` (struct) :`Vhs_CurrentTime` "+00000000.00:00:00.000000000"))))

(event `/Game/HorrorEngine/Blueprints/Core/HorrorEngineInterface.RestoreSaveData`
  (params (AssetSave :type "/Game/HorrorEngine/Blueprints/Structures/SaveStructures/AssetsSave Structure"))
  (bind ((`BooleanSlot01_63_ED79FB5D49E9ED6768D7AE96EDFDE8DB` _booleanslot01) (`BooleanSlot02_64_3DE3E28A45CAE9F3E913659977556562` _booleanslot02) (`BooleanSlot03_65_04AA048C42686C9D2AF003962AEB7F6C` _booleanslot03) (`BooleanSlot04_66_3CB4510F40F5DDD3D81BCEA77398809A` _booleanslot04)) (break `/Game/HorrorEngine/Blueprints/Structures/SaveStructures/AssetsSave` AssetSave))
  ;[1 1 1] Save Fuctions
  (set `self.Open` _booleanslot01)
  (set `self.Locked` _booleanslot02)
  (set `self.PlayerHasKey` _booleanslot03)
  (set `self.SliderLocked` _booleanslot04)
  (if (`self.Locked`)
    (`self.K2_DestroyActor`)))

(fn `UserConstructionScript`
  (bind (_boxextent_x _boxextent_y _boxextent_z) (`KismetMathLibrary.BreakVector` (`self.BoxExtent`)))
  (`BoxComponent.SetBoxExtent` (`self.Box`) (`self.BoxExtent`) true)
  (`SceneComponent.K2_AddRelativeLocation` (`self.Box`) (`KismetMathLibrary.MakeVector` 0.0 0.0 _boxextent_z) false false)
  (set `/Game/QuestManager/Blueprints/Components/Manager_QuestTarget.TargetName` (`self.TargetName`) (`self.Manager_QuestTarget`)))