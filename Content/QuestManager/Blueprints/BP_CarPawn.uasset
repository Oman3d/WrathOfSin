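; Drivable car pawn with throttle, brake, steering, handbrake, brake lights and a self-recentering orbit camera.
; Quest-target interactions finish objectives: the gas tank adds gas and enables the driver seat, which triggers EnterCar.
; EnterCar hides and attaches the player's pawn, then possesses the car.
; F runs ExitCar, which line-traces left then right for space, repossesses that pawn, and reconstructs quest manager essentials, as entry does.
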(event `InputAxis|MoveForward`
  (params (AxisValue :type "Float (single-precision)"))
  (bind _vehiclemovementcomponent (`self.VehicleMovementComponent`))
  (bind _vehiclemovementcomponent_2 (`self.VehicleMovementComponent`))
  ;[1 1 1] Movement control
  (if (>= AxisValue 0.0)
    (`ChaosVehicleMovementComponent.SetThrottleInput` _vehiclemovementcomponent_2 AxisValue)
    (`ChaosVehicleMovementComponent.SetBrakeInput` _vehiclemovementcomponent_2 0.0)
    (`/Engine/EditorBlueprintResources/StandardMacros.DoOnce` false :!label _label
      (:`Completed`
        (`self.BrakeLights` false)))
    (else
      (`ChaosVehicleMovementComponent.SetBrakeInput` _vehiclemovementcomponent (* AxisValue -1.0))
      (`ChaosVehicleMovementComponent.SetThrottleInput` _vehiclemovementcomponent 0.0)
      (`self.BrakeLights` true)
      (goto _label :!via `Reset`))))

(event `InputAxis|MoveRight`
  (params (AxisValue :type "Float (single-precision)"))
  ;[1 1 1] Movement control
  (`ChaosVehicleMovementComponent.SetSteeringInput` (`self.VehicleMovementComponent`) AxisValue))

(event `self.ReceiveTick`
  (params (DeltaSeconds :type "Float (single-precision)"))
  ;[1 1 1] Movement control
)

(event `InputAction|Handbrake`
  (params (Key :type "Key Structure"))
  (bind _vehiclemovementcomponent (`self.VehicleMovementComponent`))
  ;[1 1 1] Movement control
  (:`Pressed`
    (`ChaosVehicleMovementComponent.SetHandbrakeInput` _vehiclemovementcomponent true)
    (`self.BrakeLights` true))
  (:`Released`
    (`ChaosVehicleMovementComponent.SetHandbrakeInput` _vehiclemovementcomponent false)
    (`self.BrakeLights` false)))

(event `InputAxis|LookRight`
  (params (AxisValue :type "Float (single-precision)"))
  (bind _returnvalue (`self.GetController`))
  (bind _springarm (`self.SpringArm`))
  (bind (_relativerotation_roll _relativerotation_pitch _relativerotation_yaw) (`KismetMathLibrary.BreakRotator` (`SceneComponent.RelativeRotation` (`self.SpringArm`))))
  ;[1 1 1] Camera Control
  (if (!= AxisValue 0.0)
    (`SceneComponent.K2_AddLocalRotation` _springarm (`KismetMathLibrary.MakeRotator` 0.0 0.0 AxisValue) false false) ; Rotate camera around the vehicle
    (else
      (`SceneComponent.K2_SetRelativeRotation` _springarm (`KismetMathLibrary.MakeRotator` 0.0 0.0 (`KismetMathLibrary.FInterpTo` _relativerotation_yaw 0.0 (`GameplayStatics.GetWorldDeltaSeconds`) 1.0)) false false) ; Reset camera to original angle
    ))
  (`/Engine/EditorBlueprintResources/StandardMacros.IsValid` _returnvalue
    (:`Is Valid`
      (`Controller.SetControlRotation` _returnvalue (`SceneComponent.K2_GetComponentRotation` (`self.SpringArm`))))))

(event `self.Manager_QuestTarget.On_QuestTarget_Interacted`
  (params (OverlappedBoxTag :type Name) (ByPawn :type "Pawn Object Reference"))
  (switch `name` OverlappedBoxTag
    (:`GasTank`
      (`/Game/QuestManager/Blueprints/Components/Manager_QuestTarget.Try_Finish_Objective` (`self.Manager_QuestTarget`) "RefillCar" ByPawn)
      (set `self.Gas` (+ (`self.Gas`) 1.0))
      (if (>= (`self.Gas`) 0.0)
        (`/Game/QuestManager/Blueprints/Components/Manager_QuestTarget.Set_Interaction_Enabled` (`self.Manager_QuestTarget`) "DriverSeat" true)))
    (:`DriverSeat`
      (`/Game/QuestManager/Blueprints/Components/Manager_QuestTarget.Try_Finish_Objective` (`self.Manager_QuestTarget`) "EnterCar" ByPawn)
      (`self.EnterCar`))))

(event `self.Manager_QuestTarget.On_Manager_Constructed`)

(event `Key|F`
  (params (Key :type "Key Structure"))
  (:`Pressed`
    (`self.ExitCar`)))

(fn `BrakeLights`
  (params (BrakeLights :type Boolean))
  (bind _returnvalue (`KismetMaterialLibrary.CreateDynamicMaterialInstance` "/Game/QuestManager/Pawns/SportsCar/Materials/MI_SportsCar_Chassis.MI_SportsCar_Chassis" "None"))
  (`PrimitiveComponent.SetMaterial` (`self.Mesh`) 1 _returnvalue)
  (if BrakeLights
    (`MaterialInstanceDynamic.SetScalarParameterValue` _returnvalue "BrakeLightPower" 200.0)
    (else
      (`MaterialInstanceDynamic.SetScalarParameterValue` _returnvalue "BrakeLightPower" 4.0))))

(fn `EnterCar`
  (`|ExecutionSequence`
    (:`then_0`
      (set `self.LastControlledPawn` (`Controller.K2_GetPawn` (`GameplayStatics.GetPlayerController` 0)))
      (bind _ascharacter_movement_component (cast `CharacterMovementComponent` (`self.GetMovementComponent` (`self.LastControlledPawn`))))
      (`CharacterMovementComponent.SetMovementMode` _ascharacter_movement_component "MOVE_None" 0)
      (`self.SetActorEnableCollision` (`self.LastControlledPawn`) false)
      (`self.SetActorHiddenInGame` (`self.LastControlledPawn`) true)
      (`self.K2_AttachToActor` (`self.LastControlledPawn`) self "None" "SnapToTarget" "SnapToTarget" "KeepRelative" true))
    (:`then_1`
      (`Controller.Possess` (`GameplayStatics.GetPlayerController` 0) self)
      (bind _returnvalue (`/Game/QuestManager/Blueprints/Data/Libraries/ML_MissionComponent.Get_Quest_Manager` (`GameplayStatics.GetPlayerController` 0))
        (:`then`
          (`/Game/QuestManager/Blueprints/Components/Manager_Mission.Construct_Essentials` _returnvalue))))
    (:`then_2`
      (`/Game/QuestManager/Blueprints/Components/Manager_QuestTarget.Set_Interaction_Enabled` (`self.Manager_QuestTarget`) "DriverSeat" false))))

(fn `ExitCar`
  (locals (LocObjects :type "Array of EObjectTypeQuery Enum") (LocCanExitLeft :type Boolean) (LocCanExitRight :type Boolean))
  (bind _exitright (`self.ExitRight`))
  (bind _exitleft (`self.ExitLeft`))
  (`|ExecutionSequence`
    (:`then_0`
      (bind (_outhit _returnvalue) (`KismetSystemLibrary.LineTraceSingleForObjects` :`Start` (+ (`SceneComponent.K2_GetComponentLocation` _exitleft) (* (`SceneComponent.GetRightVector` _exitleft) 100.0)) :`End` (`SceneComponent.K2_GetComponentLocation` (`self.ExitLeft`)) :`ObjectTypes` (`local.LocObjects`) :`DrawDebugType` "ForDuration"))
      (if _returnvalue
        (bind (_outhit_2 _returnvalue_2) (`KismetSystemLibrary.LineTraceSingleForObjects` :`Start` (+ (`SceneComponent.K2_GetComponentLocation` _exitright) (* (`SceneComponent.GetRightVector` _exitright) -100.0)) :`End` (`SceneComponent.K2_GetComponentLocation` (`self.ExitRight`)) :`ObjectTypes` (`local.LocObjects`) :`DrawDebugType` "ForDuration"))
        (if (not _returnvalue_2)
          (set `local.LocCanExitRight` true)
          (`MovementComponent.StopMovementImmediately` (`self.VehicleMovementComponent`)))
        (else
          (set `local.LocCanExitLeft` true))))
    (:`then_1`
      (if (`local.LocCanExitLeft`)
        (`self.K2_DetachFromActor` (`self.LastControlledPawn`) "KeepRelative" "KeepRelative" "KeepRelative")
        (`self.K2_SetActorLocation` (`self.LastControlledPawn`) (`SceneComponent.K2_GetComponentLocation` (`self.ExitLeft`)) false true)
        (`self.SetActorHiddenInGame` (`self.LastControlledPawn`) false :!label _label)
        (`self.SetActorEnableCollision` (`self.LastControlledPawn`) true)
        (`Controller.Possess` (`GameplayStatics.GetPlayerController` 0) (`self.LastControlledPawn`))
        (bind _returnvalue_3 (`/Game/QuestManager/Blueprints/Data/Libraries/ML_MissionComponent.Get_Quest_Manager` (`GameplayStatics.GetPlayerController` 0))
          (:`then`
            (`/Game/QuestManager/Blueprints/Components/Manager_Mission.Construct_Essentials` _returnvalue_3)
            (`/Game/QuestManager/Blueprints/Components/Manager_QuestTarget.Set_Interaction_Enabled` (`self.Manager_QuestTarget`) "DriverSeat" true)))
        (elif (`local.LocCanExitRight`)
          (`self.K2_DetachFromActor` (`self.LastControlledPawn`) "KeepRelative" "KeepRelative" "KeepRelative")
          (`self.K2_SetActorLocation` (`self.LastControlledPawn`) (`SceneComponent.K2_GetComponentLocation` (`self.ExitRight`)) false true)
          (goto _label))))))

(fn `UserConstructionScript`)