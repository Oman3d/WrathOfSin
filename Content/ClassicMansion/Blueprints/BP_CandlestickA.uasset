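; BP_CandlestickA is a candlestick prop from the ClassicMansion content with three flame particle systems and three point lights, switched lit or unlit by IsActive.
; The construction script sets the lights to LightIntensity and shows the flames when active, otherwise zeroes the lights and hides the flames.
; BeginPlay sets the particle systems' active state from IsActive, while the overlap and tick events are unused.
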(event `self.ReceiveBeginPlay`
  (`ActorComponent.SetActive` (`self.PS_CandleFlame`) (`self.IsActive`) false)
  (`ActorComponent.SetActive` (`self.ParticleSystem`) (`self.IsActive`) false)
  (`ActorComponent.SetActive` (`self.ParticleSystem1`) (`self.IsActive`) false))

(fn `UserConstructionScript`
  (bind _pointlight1 (`self.PointLight1`))
  (if (`self.IsActive`)
    (`LightComponent.SetIntensity` _pointlight1 (`self.LightIntensity`))
    (`LightComponent.SetIntensity` (`self.PointLight2`) (`self.LightIntensity`))
    (`LightComponent.SetIntensity` (`self.PointLight`) (`self.LightIntensity`))
    (`SceneComponent.SetVisibility` (`self.ParticleSystem`) true false)
    (`SceneComponent.SetVisibility` (`self.ParticleSystem1`) true false)
    (`SceneComponent.SetVisibility` (`self.PS_CandleFlame`) true false)
    (else
      (`LightComponent.SetIntensity` _pointlight1 0.0)
      (`LightComponent.SetIntensity` (`self.PointLight2`) 0.0)
      (`LightComponent.SetIntensity` (`self.PointLight`) 0.0)
      (`SceneComponent.SetVisibility` (`self.ParticleSystem`) false false)
      (`SceneComponent.SetVisibility` (`self.ParticleSystem1`) false false)
      (`SceneComponent.SetVisibility` (`self.PS_CandleFlame`) false false))))