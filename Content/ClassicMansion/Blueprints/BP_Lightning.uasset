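; BP_Lightning is an ambient storm actor that loops lightning strikes at random intervals and directions.
; Each strike randomly yaws a Cube, spawns the bolt emitter along its forward vector, and adds a temporary directional light facing back, flickered by a timeline.
; Thunder follows after a delay proportional to distance.
; ActorToHide is shown at each strike and hidden five seconds after the flash ends.
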(event `self.ReceiveBeginPlay`
  (bind _distancemult (`self.DistanceMult`))
  (bind _returnvalue (`SceneComponent.GetForwardVector` (`self.Cube`)))
  (bind (_returnvalue_x _returnvalue_y) (`KismetMathLibrary.BreakVector` (* _returnvalue (`KismetMathLibrary.MakeVector` _distancemult _distancemult 1.0))))
  (bind (_returnvalue_roll _returnvalue_pitch _returnvalue_yaw) (`KismetMathLibrary.BreakRotator` (`KismetMathLibrary.Conv_VectorToRotator` (* _returnvalue (-1.0 -1.0 -1.0)))))
  (`KismetSystemLibrary.RetriggerableDelay` (`KismetMathLibrary.RandomFloatInRange` (`self.DelayMin`) (`self.DelayMax`)) :!label _label)
  (`SceneComponent.K2_SetWorldRotation` (`self.Cube`) (`KismetMathLibrary.MakeRotator` 0.0 0.0 (`KismetMathLibrary.RandomFloatInRange` -180.0 180.0)) false false)
  (`GameplayStatics.SpawnEmitterAtLocation` "/Game/ClassicMansion/Particles/PS_Lightning.PS_Lightning" (`KismetMathLibrary.MakeVector` _returnvalue_x _returnvalue_y 4000.0))
  (bind _returnvalue_2 (`AddComponent|NODE_AddDirectionalLightComponent-0` :`RelativeTransform` (`KismetMathLibrary.MakeTransform` (0.0 0.0 0.0) (`KismetMathLibrary.MakeRotator` 0.0 -10.0 _returnvalue_yaw))))
  (`self.SetActorHiddenInGame` (`self.Actor to Hide`) false)
  (`|ExecutionSequence`
    (:`then_0`
      (`KismetSystemLibrary.RetriggerableDelay` (* _distancemult 3e-05))
      (`GameplayStatics.PlaySoundAtLocation` "/Game/ClassicMansion/Audio/Cues/SC_Lightning.SC_Lightning" (`KismetMathLibrary.MakeVector` _returnvalue_x _returnvalue_y 2000.0) (struct) 1.0 1.0 0.0 null null null null))
    (:`then_1`
      (bind (_direction _lightintensity) (`Timeline|Timeline_0` :!via `PlayFromStart`)
        (:`Update`
          (`LightComponent.SetIntensity` _returnvalue_2 _lightintensity))
        (:`Finished`
          (`ActorComponent.K2_DestroyComponent` _returnvalue_2)
          (`|ExecutionSequence`
            (:`then_0`
              (goto _label))
            (:`then_1`
              (`KismetSystemLibrary.RetriggerableDelay` 5.0)
              (`self.SetActorHiddenInGame` (`self.Actor to Hide`) true))))))))

(fn `UserConstructionScript`)