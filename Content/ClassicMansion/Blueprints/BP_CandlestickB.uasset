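; BP_CandlestickB is a candlestick prop for the Classic Mansion with a point light and a candle flame particle effect.
; Its construction script uses IsActive to light or snuff it, setting the light to LightIntensity or zero and showing or hiding the flame.
; The event graph does nothing at runtime, as its events are empty and a SetActive call on the flame is never run.
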(event `self.ReceiveBeginPlay`)

(fn `UserConstructionScript`
  (bind _ps_candleflame (`self.PS_CandleFlame`))
  (bind _pointlight (`self.PointLight`))
  (if (`self.IsActive`)
    (`LightComponent.SetIntensity` _pointlight (`self.LightIntensity`))
    (`SceneComponent.SetVisibility` _ps_candleflame true false)
    (else
      (`LightComponent.SetIntensity` _pointlight 0.0)
      (`SceneComponent.SetVisibility` _ps_candleflame false false))))