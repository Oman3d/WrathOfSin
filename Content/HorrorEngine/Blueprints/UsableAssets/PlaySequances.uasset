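; Horror Engine usable trigger that plays level sequences selected by tag when a character enters its box or its Open/On event fires.
; Open/On runs the interaction check, plays every LevelSequenceActor whose tag array exactly matches SequanceTagToPlay, then sets Open, which blocks further overlap triggers.
; Save hooks add an entry to the player's save component cache and restore the Open flag without replaying sequences.
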(event `self.Open/On`
  (params (HorrorEvent :type Boolean))
  (`/Game/HorrorEngine/Blueprints/Core/HorrorEngineMacros.HM_CheckInteraction`)
  (bind _outactors (`GameplayStatics.GetAllActorsOfClass` "/Script/LevelSequence.LevelSequenceActor"))
  (for (_array_element _array_index) _outactors
    (if (`KismetArrayLibrary.Array_Identical` (`Actor.Tags` _array_element) (`|MakeArray` (`self.SequanceTagToPlay`)))
      (`MovieSceneSequencePlayer.Play` (`LevelSequenceActor.SequencePlayer` (`|GetArrayItem` _outactors _array_index)))))
  (set `self.Open` true))

(event `self.Box.OnComponentBeginOverlap`
  (params (OverlappedComponent :type "PrimitiveComponent Object Reference") (OtherActor :type "Actor Object Reference") (OtherComp :type "PrimitiveComponent Object Reference") (OtherBodyIndex :type Integer) (bFromSweep :type Boolean) (SweepResult :type "HitResult Structure (by ref)"))
  (if (not (`self.Open`))
    (cast `/Game/MainLevels/Player/BP_CharacterBase` OtherActor)
    (`self.Open/On` false)))

(event `/Game/HorrorEngine/Blueprints/Core/HorrorEngineInterface.CollectSaveData`
  ;[0 1 0.5572] Save Settings
  (bind _asmaster (`/Game/HorrorEngine/Blueprints/Core/HorrorEngineFunctions.GetPlayer`))
  (`KismetArrayLibrary.Array_Add` (`/Game/HorrorEngine/Blueprints/Core/HE_SaveGameComponent.AssetCache` (`/Game/HorrorEngine/HorrorEngine.HE_SaveGameComponent` _asmaster)) (make `/Game/HorrorEngine/Blueprints/Structures/SaveStructures/AssetsSave` (`KismetSystemLibrary.GetObjectName` self) (`self.Open`) false false false 0.0 0.0 0 "+00000000.00:00:00.000000000" "NewEnumerator0" (struct :`Actor` "NewEnumerator0" :`MeshSettings` (struct) :`InspectionSettings` (struct :`InspectionPivotLocation` (0.0 0.0 0.0) :`Takeable` true :`InspectionAnimation` true :`InspectionAnimationSpeedSec` 0.5 :`InspectionBeginRotation` (struct) :`InspectionBeginScale` 1.0 :`MinZoomScale` 1.0 :`MaxZoomScale` 2.0 :`RotationSpeed` 2.5 :`SlideSpeed` 1.0 :`MaxSlideValue` 10.0 :`ItemName` "NSLOCTEXT(\"[F3C345104BDE59DAC9C9E29320DDAC8A]\", \"591F13DE468FFE8449A75C91E5977088\", \"Item Name\")" :`ItemInformation` "NSLOCTEXT(\"[F3C345104BDE59DAC9C9E29320DDAC8A]\", \"3291CD7442C9D058E27C978C71FEBF4E\", \"Item Information\")" :`ReadingText` "NSLOCTEXT(\"[F3C345104BDE59DAC9C9E29320DDAC8A]\", \"71356DA14E0A1AC1148B64A85E7EAB8A\", \"Reading Text\")" :`TakeButton` (struct :`ButtonText` "NSLOCTEXT(\"[F3C345104BDE59DAC9C9E29320DDAC8A]\", \"090412D748C5E6B0228979B2448B59C8\", \"Take\")") :`ExamineButton` (struct :`ButtonText` "NSLOCTEXT(\"[F3C345104BDE59DAC9C9E29320DDAC8A]\", \"EDA79A08451EECB8A653F78AECD9170A\", \"Examine\")") :`ZoomSlideButton` (struct :`ButtonText` "NSLOCTEXT(\"[F3C345104BDE59DAC9C9E29320DDAC8A]\", \"08CA27434485FF71D71CA0B04D6AA2FE\", \"Zoom/Slide\")") :`DismissButton` (struct :`ButtonText` "NSLOCTEXT(\"[F3C345104BDE59DAC9C9E29320DDAC8A]\", \"A06C807A4255530CEFC9FA93ECD14DA3\", \"Dismiss\")")) :`InventorySettings` (struct :`StorageType` "NewEnumerator3" :`NumberofItemstoAddInventory` 1 :`Interactable` true :`InteractionButton` (struct :`ButtonText` "NSLOCTEXT(\"[F3C345104BDE59DAC9C9E29320DDAC8A]\", \"6BFA5A8146582528DE3A4EB9A26E83A4\", \"Use\")") :`SwitchButton` (struct :`ButtonText` "NSLOCTEXT(\"[F3C345104BDE59DAC9C9E29320DDAC8A]\", \"3D264310437B212A2E067B92139E1800\", \"Switch\")") :`ZoomSlideButton` (struct :`ButtonText` "NSLOCTEXT(\"[F3C345104BDE59DAC9C9E29320DDAC8A]\", \"40A9D612421406157D1D629D16517E82\", \"Zoom/Slide\")") :`CloseInventoryButton` (struct :`ButtonText` "NSLOCTEXT(\"[F3C345104BDE59DAC9C9E29320DDAC8A]\", \"A48252244DC7005308BB2F922B749487\", \"Close\")")) :`Pistol_MeshSettingsTop` (struct) :`Vhs_CurrentTime` "+00000000.00:00:00.000000000"))))

(event `/Game/HorrorEngine/Blueprints/Core/HorrorEngineInterface.RestoreSaveData`
  (params (AssetSave :type "/Game/HorrorEngine/Blueprints/Structures/SaveStructures/AssetsSave Structure"))
  ;[0 1 0.5572] Save Settings
  (set `self.Open` (`.BooleanSlot01_63_ED79FB5D49E9ED6768D7AE96EDFDE8DB` (break `/Game/HorrorEngine/Blueprints/Structures/SaveStructures/AssetsSave` AssetSave))))

(fn `UserConstructionScript`
  (`parent.UserConstructionScript`))