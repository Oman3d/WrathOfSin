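; Usable spawner that puts the player into a PossessedPlayer ghost and later returns them to their character.
; Use or SpawnGhost flags the character as possessed, spawns the ghost at one of seven random points and transfers controller possession to it.
; ComeBack destroys the ghost, repossesses the original character, cuts fear XP, grants faith XP and calls Alive.
; Weighted item-picking functions are defined but not called by these events.
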(event `Comback to Life`
  (bind _returnvalue (`GameplayStatics.GetPlayerController` 0))
  (bind (_fearsystem_currentfearlevel _fearsystem_fearxp _fearsystem_neededfearxp _fearsystem_levelcap _fearsystem_currentxp _fearsystem_currentmaxxp _fearsystem_currentpercentage _fearsystem_bufferxp) (break `/Game/HorrorEngine/Blueprints/Structures/FearSystem` (`/Game/MainLevels/Player/BP_CharacterBase.FearSystem` (`self.Player ref`))))
  (bind (_faith_system_struct_currentfaithlevel _faith_system_struct_faithxp _faith_system_struct_neededfaithxp _faith_system_struct_levelcap _faith_system_struct_currentxp _faith_system_struct_currentmaxxp _faith_system_struct_currentpercentage _faith_system_struct_bufferxp) (break `/Game/HorrorEngine/Blueprints/Structures/FaithSystem` (`/Game/MainLevels/Player/BP_CharacterBase.Faith System Struct` (`self.Player ref`))))
  (`self.K2_DestroyActor` (`self.Ghost Ref`))
  (bind _outactors (`GameplayStatics.GetAllActorsOfClass` "/Game/MainLevels/Player/BP_CharacterBase.BP_CharacterBase_C"))
  (set `self.Player ref` (`|GetArrayItem` _outactors))
  (`self.EnableInput` (`self.Player ref`) _returnvalue)
  (`Controller.Possess` _returnvalue (`self.Player ref`))
  (set `/Game/MainLevels/Player/BP_CharacterBase.FearSystem` (make `/Game/HorrorEngine/Blueprints/Structures/FearSystem` _fearsystem_currentfearlevel _fearsystem_fearxp _fearsystem_neededfearxp _fearsystem_levelcap (* _fearsystem_currentxp 0.15) _fearsystem_currentmaxxp _fearsystem_currentpercentage _fearsystem_bufferxp) (`self.Player ref`))
  (set `/Game/MainLevels/Player/BP_CharacterBase.Faith System Struct` (make `/Game/HorrorEngine/Blueprints/Structures/FaithSystem` _faith_system_struct_currentfaithlevel _faith_system_struct_faithxp _faith_system_struct_neededfaithxp _faith_system_struct_levelcap (+ _faith_system_struct_currentxp 250.0) _faith_system_struct_currentmaxxp _faith_system_struct_currentpercentage _faith_system_struct_bufferxp) (`self.Player ref`))
  (`/Game/MainLevels/Player/BP_CharacterBase.Alive` (`self.Player ref`))
  (set `/Game/MainLevels/Player/BP_CharacterBase.Player Possesed` false (`self.Player ref`)))

(event `SpawnGhost`
  (bind _returnvalue (`GameplayStatics.GetPlayerController` 0))
  (bind _outactors (`GameplayStatics.GetAllActorsOfClass` "/Game/MainLevels/Player/BP_CharacterBase.BP_CharacterBase_C" :!label _label))
  (bind _output (`|GetArrayItem` _outactors))
  (set `self.Player ref` _output)
  (set `self.actor location save` (`self.GetTransform` _output))
  (set `/Game/MainLevels/Player/BP_CharacterBase.Player Possesed` true (`self.Player ref`))
  (bind _returnvalue_2 (`|SpawnActorFromClass` "/Game/MainLevels/Player/PossessedPlayer.PossessedPlayer_C" (`SceneComponent.K2_GetComponentToWorld` (`|GetArrayItem` (`|MakeArray` (`self.SpawnPoint01`) (`self.SpawnPoint02`) (`self.SpawnPoint03`) (`self.SpawnPoint04`) (`self.SpawnPoint05`) (`self.SpawnPoint06`) (`self.SpawnPoint07`)) (`KismetMathLibrary.RandomIntegerInRange` 0 6))) "AdjustIfPossibleButAlwaysSpawn" "OverrideRootScale" null null))
  (set `self.Ghost Ref` _returnvalue_2)
  (`self.EnableInput` (`self.Ghost Ref`) _returnvalue)
  (`Controller.Possess` _returnvalue (`self.Ghost Ref`)))

(event `self.Use`
  (params (HorrorEvent :type Boolean))
  (goto _label))

(event `ComeBack`
  (`self.Comback to Life`))

(fn `CalulateSum`
  (returns (`Total Sum` :type "Float (double-precision)"))
  (locals (RunningTotal :type "Float (double-precision)"))
  (bind _values (`BlueprintMapLibrary.Map_Values` (`self.Item To Spawm`)))
  (for _array_element _values
    (set `local.RunningTotal` (+ (`local.RunningTotal`) _array_element)))
  (return (`local.RunningTotal`)))

(fn `Choose Item`
  (returns (Item :type "Actor Class Reference"))
  (locals (RandomValue :type "Float (double-precision)" :default 0.0))
  (set `local.RandomValue` (`KismetMathLibrary.RandomFloatInRange` 0.0 (`self.Value Sum`)))
  (bind _keys (`BlueprintMapLibrary.Map_Keys` (`self.Item To Spawm`)))
  (for _array_element _keys
    (bind _value (`BlueprintMapLibrary.Map_Find` (`self.Item To Spawm`) _array_element))
    (if (< (`local.RandomValue`) _value)
      (return _array_element)
      (else
        (set `local.RandomValue` (- (`local.RandomValue`) _value))))))

(fn `Item Selector`
  (params (`Item Integer` :type Integer))
  (returns (`Item To Spawn` :type "Actor Class Reference"))
  (bind _keys (`BlueprintMapLibrary.Map_Keys` (`self.Item To Spawm`)))
  (return (`|GetArrayItem` _keys `Item Integer`)))

(fn `UserConstructionScript`)