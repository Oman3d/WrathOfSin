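; AreaSpawnBounds is a named box volume that tracks whether a BP_CharacterBase is inside it, apparently to mark an area for spawning.
; A looping one-second timer runs an overlap query on the RandomAreaSpawn box to set InBounds, while its begin and end overlap events separately toggle Overlaped.
; The construction script sizes the box and cube from BoxCollectionScale, tags the actor with AreaName and displays that name as text raised by the box's height extent.
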(event `self.ReceiveBeginPlay`
  (bind _returnvalue (`KismetSystemLibrary.K2_SetTimer` null "Check for Player " 1.0 true))
  (set `self.Timer` _returnvalue))

(event `Check for Player`
  (bind _random_area_spawn (`self.Random area Spawn`))
  (bind (_outactors _returnvalue) (`KismetSystemLibrary.ComponentOverlapActors` _random_area_spawn (`SceneComponent.K2_GetComponentToWorld` _random_area_spawn) (`self.Object Types_0`) "/Game/MainLevels/Player/BP_CharacterBase.BP_CharacterBase_C"))
  (if _returnvalue
    (set `self.In Bounds` true)
    (else
      (set `self.In Bounds` false))))

(event `self.Random area Spawn.OnComponentBeginOverlap`
  (params (OverlappedComponent :type "PrimitiveComponent Object Reference") (OtherActor :type "Actor Object Reference") (OtherComp :type "PrimitiveComponent Object Reference") (OtherBodyIndex :type Integer) (bFromSweep :type Boolean) (SweepResult :type "HitResult Structure (by ref)"))
  (cast `/Game/MainLevels/Player/BP_CharacterBase` OtherActor)
  (set `self.Overlaped` true))

(event `self.Random area Spawn.OnComponentEndOverlap`
  (params (OverlappedComponent :type "PrimitiveComponent Object Reference") (OtherActor :type "Actor Object Reference") (OtherComp :type "PrimitiveComponent Object Reference") (OtherBodyIndex :type Integer))
  (cast `/Game/MainLevels/Player/BP_CharacterBase` OtherActor)
  (set `self.Overlaped` false))

(fn `UserConstructionScript`
  (bind _box_collection_scale (`self.Box Collection Scale`))
  (bind _random_area_spawn (`self.Random area Spawn`))
  (`BoxComponent.SetBoxExtent` _random_area_spawn _box_collection_scale true)
  (`SceneComponent.SetWorldScale3D` (`self.Cube`) (* _box_collection_scale 0.0199))
  (`SceneComponent.K2_SetRelativeLocation` (`self.TextRender`) (`KismetMathLibrary.MakeVector` 0.0 0.0 (.z (`.BoxExtent` (`KismetSystemLibrary.GetComponentBounds` _random_area_spawn)))) false true)
  (bind _output_get (set `self.Tags` (`|MakeArray` (`self.Area name_`))))
  (`TextRenderComponent.K2_SetText` (`self.TextRender`) (`KismetTextLibrary.Conv_NameToText` (`|GetArrayItem` _output_get))))