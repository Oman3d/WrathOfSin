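; EnemySpawnPoint is a spawn point marker actor in HorrorEngine that shows its first actor tag as text and turns toward the player.
; The construction script writes that tag into a TextRender component, while the file itself contains no spawning logic.
; A looping one-second timer started on BeginPlay, rather than Tick, sets the actor's yaw toward the player character when within 2000 units.
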(event `self.ReceiveBeginPlay`
  (`KismetSystemLibrary.K2_SetTimer` null "Face Player" 1.0 true))

(event `Face Player`
  (bind _returnvalue (`GameplayStatics.GetPlayerCharacter` 0))
  (bind (_returnvalue_roll _returnvalue_pitch _returnvalue_yaw) (`KismetMathLibrary.BreakRotator` (`KismetMathLibrary.FindLookAtRotation` (`self.K2_GetActorLocation`) (`self.K2_GetActorLocation` _returnvalue))))
  (if (<= (`self.GetDistanceTo` _returnvalue) 2000.0)
    (`self.K2_SetActorRotation` (`KismetMathLibrary.MakeRotator` 0.0 0.0 _returnvalue_yaw))))

(fn `UserConstructionScript`
  (`TextRenderComponent.K2_SetText` (`self.TextRender`) (`KismetTextLibrary.Conv_NameToText` (`|GetArrayItem` (`self.Tags`)))))