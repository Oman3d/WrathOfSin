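; TheLight is a trigger actor that acts as the player's escape from the nightmare world.
; When a PossessedPlayer overlaps its sphere, it flags them as saved, disables input and fades the camera to black.
; After a delay it calls ComeBack on the first PossesedPlayerSpawner found in the world, fades the camera back and unloads the NightMareWorld streaming level.
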(event `self.ReceiveBeginPlay`)

(event `self.Sphere.OnComponentBeginOverlap`
  (params (OverlappedComponent :type "PrimitiveComponent Object Reference") (OtherActor :type "Actor Object Reference") (OtherComp :type "PrimitiveComponent Object Reference") (OtherBodyIndex :type Integer) (bFromSweep :type Boolean) (SweepResult :type "HitResult Structure (by ref)"))
  (bind _aspossessed_player (cast `/Game/MainLevels/Player/PossessedPlayer` OtherActor))
  (set `/Game/MainLevels/Player/PossessedPlayer.ImSaved` true _aspossessed_player)
  (`self.DisableInput` _aspossessed_player (`GameplayStatics.GetPlayerController` 0))
  (`/Game/FPS_Game/Blueprints/System/BP_Library.CameraFadeToBlack` 4.0)
  (`KismetSystemLibrary.Delay` 5.0)
  (bind _outactors (`GameplayStatics.GetAllActorsOfClass` "/Game/HorrorEngine/Blueprints/UsableAssets/PossesedPlayerSpawner.PossesedPlayerSpawner_C"))
  (`/Game/HorrorEngine/Blueprints/UsableAssets/PossesedPlayerSpawner.ComeBack` (`|GetArrayItem` _outactors))
  (`/Game/FPS_Game/Blueprints/System/BP_Library.CameraFadeToDefault` 3.0)
  (`GameplayStatics.UnloadStreamLevel` "NightMareWorld"))

(fn `UserConstructionScript`)