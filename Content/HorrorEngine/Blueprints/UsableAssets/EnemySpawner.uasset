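; Horror Engine usable spawner that spawns a set number of zombies or bosses when switched on, firing a horror event when none remain.
; Looping timers drive spawning, remaining-enemy checks and AreaSpawnBounds checks that despawn enemies outside and resume spawning from the saved count inside.
; Tagged or all EnemySpawnPoints are filtered by player distance, elevation and off-screen tests.
; Optional chase mode teleports distant enemies to those nearby points.
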(event `EnemyCheck`
  ;[1 1 1] Check for Enemys left
  (if (<= (`KismetArrayLibrary.Array_Length` (`self.Active Zombie array`)) 0)
    (`self.HorrorEventCheck` "NewEnumerator4")
    (`KismetSystemLibrary.K2_ClearTimer` null "EnemyCheck")))

(event `update enemy check`)

(event `SpawnEnemys`
  ;[1 1 1] Spawning Fuctions
  (`self.Get Points Near Player`)
  (`self.Get Random Point to Spawn`)
  (if (`self.Dont Move`)
    _
    (elif (`KismetMathLibrary.ClassIsChildOf` (`self.WhoToSpawn`) "/Game/MainLevels/Enemys/Ai/BaseBoss.BaseBoss_C")
      (bind _outactors (`GameplayStatics.GetAllActorsOfClass` "/Game/MainLevels/Enemys/Ai/BaseBoss.BaseBoss_C"))
      (if (<= (`KismetArrayLibrary.Array_Length` _outactors) (- (`self.How many to Spawn`) 1))
        (`KismetSystemLibrary.Delay` (`self.Delay Between Spawns`))
        (`self.SingleSpawn` (`self.WhoToSpawn`))
        (elif (not (`self.Respawn Enemy?`))
          (`KismetSystemLibrary.K2_PauseTimerHandle` (`self.SpawnEnemy Timer Ref`))
          (set `self.Spawned` true)
          (`self.Save Enemys`)))
      (else
        (bind _outactors_2 (`GameplayStatics.GetAllActorsOfClass` "/Game/MainLevels/Enemys/Ai/BaseZombie.BaseZombie_C"))
        (if (<= (`KismetArrayLibrary.Array_Length` _outactors_2) (- (`self.How many to Spawn`) 1))
          (`KismetSystemLibrary.Delay` (`self.Delay Between Spawns`))
          (switch `/Game/HorrorEngine/Blueprints/Enums/SpawnType` (`self.Spawn Location`)
            (:`NewEnumerator0`
              (`self.SingleSpawn` (`self.WhoToSpawn`)))
            (:`NewEnumerator1`
              (`self.Multi Spawn` (`self.WhoToSpawn`))))
          (`self.RespawnEnemys`)
          (elif (not (`self.Respawn Enemy?`))
            (`KismetSystemLibrary.K2_PauseTimerHandle` (`self.SpawnEnemy Timer Ref`))
            (set `self.Spawned` true)
            (`self.Save Enemys`)))))))

(event `Move closer to player`
  ;[1 1 1] Chase Player Fuctions
  (`self.Get Points Near Player`)
  (`self.Get Random Point to Spawn`)
  (`KismetSystemLibrary.Delay` (`self.Delay Between Spawns`))
  (if (not (`self.Dont Move`))
    (`self.Spawn Enemy near Player`)))

(event `self.ReceiveBeginPlay`
  (bind _returnvalue (`GameplayStatics.GetPlayerCharacter` 0))
  ;[1 1 1] BegainFuctions
  (`self.Set Area Bounds`)
  (`self.Get Spawn points`)
  (bind _asbp_character_base (cast `/Game/MainLevels/Player/BP_CharacterBase` _returnvalue)
    (:`then`
      (set `self.As BP Character Base` _asbp_character_base))
    (:`CastFailed`
      (bind _aspossessed_player (cast `/Game/MainLevels/Player/PossessedPlayer` _returnvalue))
      (set `self.As BP Character Base` _aspossessed_player)))
  (if (`self.Spawn on Play`)
    (`self.Open/On` false)))

(event `self.Open/On`
  (params (HorrorEvent :type Boolean))
  (bind _delay_between_spawns (`self.Delay Between Spawns`))
  ;[1 1 1] Open Fuctions
  (`KismetSystemLibrary.PrintString` (`KismetSystemLibrary.GetDisplayName` self))
  (`/Game/HorrorEngine/Blueprints/Core/HorrorEngineMacros.HM_CheckInteraction`)
  (bind _returnvalue (`KismetSystemLibrary.K2_SetTimer` null "SpawnEnemys" _delay_between_spawns true))
  (set `self.SpawnEnemy Timer Ref` _returnvalue)
  (`KismetSystemLibrary.K2_SetTimer` null "EnemyCheck" 7.0 true)
  (`KismetSystemLibrary.K2_SetTimer` null "Is Player In Bounds" 1.0 true)
  (if (`self.Enemy Chase Player `)
    (`KismetSystemLibrary.K2_SetTimer` null "Move closer to player" _delay_between_spawns true)))

(event `self.Close/Off`
  (params (HorrorEvent :type Boolean))
  ;[1 1 1] Close Fuctions
  (`/Game/HorrorEngine/Blueprints/Core/HorrorEngineMacros.HM_CheckInteraction`)
  (`KismetSystemLibrary.K2_ClearTimer` null "SpawnEnemys")
  (for _array_element (`self.Active Zombie array`)
    (`self.K2_DestroyActor` _array_element))
  (`self.HorrorEventCheck` "NewEnumerator4"))

(event `Remove active Enemys`
  ;[1 1 1] Remove active Enemys
  (`KismetSystemLibrary.Delay` 0.2)
  (for _array_element (`self.Active Zombie array`)
    (`self.K2_DestroyActor` _array_element)
    (`KismetArrayLibrary.Array_RemoveItem` (`self.Active Zombie array`) _array_element)))

(event `Is Player In Bounds`
  ;[1 1 1] Check Bounds
  (`self.Set Area Bounds`)
  (`self.Check Area Bounds`))

(event `/Game/MainLevels/Enemys/Ai/EnemyDead.Enemy Dead`
  (params (NewParam :type "Actor Object Reference"))
  ;[1 1 1] Removes Dead Enemys
  (bind _returnvalue (`KismetArrayLibrary.Array_RemoveItem` (`self.Active Zombie array`) NewParam))
  (`self.Save Enemys`)
  (if _returnvalue
    (`KismetSystemLibrary.PrintString` "fart")
    (for _array_element (`self.Active Zombie array`)
      (`KismetSystemLibrary.PrintString` (`KismetSystemLibrary.GetDisplayName` _array_element) true true (struct :`R` 1.0 :`G` 0.770742 :`B` 0.167383 :`A` 1.0)))))

(event `Spawn Saved Enemys`
  ;[1 1 1] Spawn Saved Enemy
  (set `self.How many to Spawn` (`KismetArrayLibrary.Array_Length` (`self.Save Zombie array`)))
  (`KismetSystemLibrary.K2_UnPauseTimerHandle` (`self.SpawnEnemy Timer Ref`))
  (`KismetSystemLibrary.Delay` 0.2))

(event `Save Enemys`
  ;[1 1 1] Save Enemys Left
  (`KismetArrayLibrary.Array_Clear` (`self.Save Zombie array`))
  (for _array_element (`self.Active Zombie array`)
    (`KismetArrayLibrary.Array_Add` (`self.Save Zombie array`) _array_element)
    (for _array_element_2 (`self.Save Zombie array`)
      (`KismetSystemLibrary.PrintString` (`KismetSystemLibrary.GetDisplayName` _array_element_2)))))

(fn `Add to Spawn height`
  (params (InTransform :type "Transform Structure (by ref)"))
  (returns (ReturnValue :type "Transform Structure"))
  (return (`KismetMathLibrary.MakeTransform` (`KismetMathLibrary.MakeVector` (.x (.location InTransform)) (.y (.location InTransform)) (+ (.z (.location InTransform)) 100.0)) (.rotation InTransform) (.scale InTransform))))

(fn `Check Area Bounds`
  (if (`KismetArrayLibrary.Array_Contains` (`self.Inbounds Array`) true)
    (if (`self.Spawned`)
      (`KismetSystemLibrary.PrintString` "Im In Side")
      (`self.Spawn Saved Enemys`))
    (elif (`KismetArrayLibrary.Array_Contains` (`self.Overlaped`))
      (`KismetSystemLibrary.PrintString` "Im not  Side")
      (`self.Remove active Enemys`))))

(fn `Get Points Near Player`
  (bind (_returnvalue_x _returnvalue_y) (`KismetMathLibrary.BreakVector2D` (`WidgetLayoutLibrary.GetViewportSize`)))
  (bind _spawn_point_hight_range (`self.Spawn Point Hight Range`))
  (bind _spawn_point_near_player_ (`self.Spawn point near Player `))
  (bind _spawn_point_near_player__2 (`self.Spawn point near Player `))
  (bind _spawnpoints_in_range (`self.SpawnPoints In Range`))
  (bind (_returnvalue_x_2 _returnvalue_y_2 _returnvalue_z) (`KismetMathLibrary.BreakVector` (`self.K2_GetActorLocation` (`self.Spawn point near Player `))))
  (bind (_returnvalue_x_3 _returnvalue_y_3 _returnvalue_z_2) (`KismetMathLibrary.BreakVector` (`self.K2_GetActorLocation` (`self.As BP Character Base`))))
  (bind _screenlocation (`PlayerController.ProjectWorldLocationToScreen` (`GameplayStatics.GetPlayerController` 0) (`self.K2_GetActorLocation`) false))
  (if (not (<= (`KismetArrayLibrary.Array_Length` _spawnpoints_in_range) 0))
    (for _array_element _spawnpoints_in_range
      (bind _output_get (set `self.Spawn point near Player ` _array_element))
      (if (and (<= (`self.GetDistanceTo` _output_get (`self.As BP Character Base`)) (`self.Range to Player`)) (`KismetMathLibrary.InRange_FloatFloat` _returnvalue_z (- _returnvalue_z_2 _spawn_point_hight_range) (+ _returnvalue_z_2 _spawn_point_hight_range)) (not (and (> (`KismetMathLibrary.BreakVector2D` _screenlocation) 0.0) (< (`KismetMathLibrary.BreakVector2D` _screenlocation) _returnvalue_x) (> (`.Y` (`KismetMathLibrary.BreakVector2D` _screenlocation)) 0.0) (< (`.Y` (`KismetMathLibrary.BreakVector2D` _screenlocation)) _returnvalue_y))))
        (`/Engine/EditorBlueprintResources/StandardMacros.IsValid` _spawn_point_near_player__2
          (:`Is Valid`
            (`KismetArrayLibrary.Array_Add` (`self.Spawn Points Near Player`) _spawn_point_near_player__2)))
        (else
          (`/Engine/EditorBlueprintResources/StandardMacros.IsValid` _spawn_point_near_player_
            (:`Is Valid`
              (`KismetArrayLibrary.Array_RemoveItem` (`self.Spawn Points Near Player`) _spawn_point_near_player_))))))
    (return)))

(fn `Get Random Point to Spawn`
  (returns (ReturnValue :type "Transform Structure (by ref)"))
  (bind _spawn_points_near_player (`self.Spawn Points Near Player`))
  (bind _output (`|GetArrayItem` _spawn_points_near_player (`self.SpawnPoint index`)))
  (`/Engine/EditorBlueprintResources/StandardMacros.IsValid` _output
    (:`Is Valid`
      (set `self.Dont Move` false)
      (set `self.Location to spawn` (`self.Add to Spawn height` (`SceneComponent.K2_GetComponentToWorld` (`Actor.RootComponent` _output))))
      (if (>= (`self.SpawnPoint index`) (- (`KismetArrayLibrary.Array_Length` _spawn_points_near_player) 1))
        (set `self.SpawnPoint index` 0)
        (else
          (`/Engine/EditorBlueprintResources/StandardMacros.IncrementInt` (`self.SpawnPoint index`)
            (:`  `
              (return (`self.Location to spawn`)))))))
    (:`Is Not Valid`
      (set `self.Dont Move` true))))

(fn `Get Spawn points`
  (switch `/Game/MainLevels/BluePrints/SpawnCollectionToUse` (`self.Spawn Collection to Use`)
    (:`NewEnumerator1`
      (bind _outactors (`GameplayStatics.GetAllActorsOfClass` "/Game/HorrorEngine/Blueprints/UsableAssets/EnemySpawnPoint.EnemySpawnPoint_C"))
      (for _array_element _outactors
        (if (== (`|GetArrayItem` (`Actor.Tags` _array_element)) (`self.Area / Spawn Point Tag`))
          (`KismetArrayLibrary.Array_Add` (`self.SpawnPoints In Range`) _array_element))))
    (:`NewEnumerator2`
      (bind _outactors_2 (`GameplayStatics.GetAllActorsOfClass` "/Game/HorrorEngine/Blueprints/UsableAssets/EnemySpawnPoint.EnemySpawnPoint_C"))
      (set `self.SpawnPoints In Range` _outactors_2)))
  (return))

(fn `Multi Spawn`
  (params (Class :type "Actor Class Reference"))
  (bind _returnvalue (`|SpawnActorFromClass` Class (`self.Location to spawn`) "AdjustIfPossibleButAlwaysSpawn" "OverrideRootScale" null null))
  (`KismetArrayLibrary.Array_Add` (`self.Active Zombie array`) _returnvalue)
  (return))

(fn `RandomSpawn`
  (params (Class :type "Actor Class Reference")))

(fn `RespawnEnemys`
  (if (`self.Respawn Enemy?`)
    (bind _outactors (`GameplayStatics.GetAllActorsOfClass` "/Game/MainLevels/Enemys/Ai/BaseZombie.BaseZombie_C"))
    (if (<= (`KismetArrayLibrary.Array_Length` _outactors) (`self.How many to Spawn`))
      (`KismetSystemLibrary.K2_SetTimer` null "Spawn Enemts" (`self.Delay Between Spawns`) true)
      (return))
    (else
      (return))))

(fn `Set Area Bounds`
  (bind _array_element (`self.Array Element`))
  (bind _array_element_2 (`self.Array Element`))
  (switch `/Game/MainLevels/BluePrints/SpawnCollectionToUse` (`self.Spawn Collection to Use`)
    (:`NewEnumerator1`
      ;[1 1 1] Get Specified Area Bounds
      (bind _outactors (`GameplayStatics.GetAllActorsOfClass` "/Game/HorrorEngine/Blueprints/UsableAssets/AreaSpawnBounds.AreaSpawnBounds_C"))
      (for (_array_element_3 _array_index) _outactors
        (set `self.Array Element` _array_element_3)
        (if (== (`|GetArrayItem` (`Actor.Tags` _array_element_3)) (`self.Area / Spawn Point Tag`))
          (`KismetArrayLibrary.Array_Set` (`self.Inbounds Array`) _array_index (`/Game/HorrorEngine/Blueprints/UsableAssets/AreaSpawnBounds.In Bounds` _array_element_2) true)
          (`KismetArrayLibrary.Array_Set` (`self.Overlaped`) _array_index (`/Game/HorrorEngine/Blueprints/UsableAssets/AreaSpawnBounds.Overlaped` _array_element_2) true)))
      (return))
    (:`NewEnumerator2`
      ;[1 1 1] Get All Area Bounds
      (bind _outactors_2 (`GameplayStatics.GetAllActorsOfClass` "/Game/HorrorEngine/Blueprints/UsableAssets/AreaSpawnBounds.AreaSpawnBounds_C"))
      (for (_array_element_4 _array_index_2) _outactors_2
        (set `self.Array Element` _array_element_4)
        (`KismetArrayLibrary.Array_Set` (`self.Inbounds Array`) _array_index_2 (`/Game/HorrorEngine/Blueprints/UsableAssets/AreaSpawnBounds.In Bounds` _array_element) true)
        (`KismetArrayLibrary.Array_Set` (`self.Overlaped`) _array_index_2 (`/Game/HorrorEngine/Blueprints/UsableAssets/AreaSpawnBounds.Overlaped` _array_element) true))
      (return))))

(fn `SingleSpawn`
  (params (Class :type "Actor Class Reference"))
  (bind _returnvalue (`|SpawnActorFromClass` Class (`SceneComponent.K2_GetComponentToWorld` (`self.Arrow`)) "AdjustIfPossibleButAlwaysSpawn" "OverrideRootScale" null null))
  (`KismetArrayLibrary.Array_Add` (`self.Active Zombie array`) _returnvalue)
  (return))

(fn `Spawn Enemy near Player`
  (locals (`Who to Move` :type "Actor Object Reference"))
  (bind (_returnvalue_x _returnvalue_y) (`KismetMathLibrary.BreakVector2D` (`WidgetLayoutLibrary.GetViewportSize`)))
  (bind _spawn_point_hight_range (`self.Spawn Point Hight Range`))
  (bind _spawn_points_near_player (`self.Spawn Points Near Player`))
  (bind (_returnvalue_x_2 _returnvalue_y_2 _returnvalue_z) (`KismetMathLibrary.BreakVector` (`self.K2_GetActorLocation` (`self.Spawn point near Player `))))
  (bind (_returnvalue_x_3 _returnvalue_y_3 _returnvalue_z_2) (`KismetMathLibrary.BreakVector` (`self.K2_GetActorLocation` (`self.As BP Character Base`))))
  (bind _screenlocation (`PlayerController.ProjectWorldLocationToScreen` (`GameplayStatics.GetPlayerController` 0) (`self.K2_GetActorLocation`) false))
  (for _array_element (`self.Active Zombie array`)
    (bind _output_get (set `self.Who to Move to` _array_element))
    (`/Engine/EditorBlueprintResources/StandardMacros.IsValid` _output_get
      (:`Is Valid`
        (if (not (<= (`self.GetDistanceTo` (`self.Who to Move to`) (`self.As BP Character Base`)) 3000.0))
          (`/Engine/EditorBlueprintResources/StandardMacros.IsValid` (`self.Who to Move to`)
            (:`Is Valid`
              (if (`self.Dont Move`)
                (set `self.Dont Move` false)
                (elif (and (>= (`self.SpawnPoint index`) (- (`KismetArrayLibrary.Array_Length` _spawn_points_near_player) 1)) (`KismetMathLibrary.InRange_FloatFloat` _returnvalue_z (- _returnvalue_z_2 _spawn_point_hight_range) (+ _returnvalue_z_2 _spawn_point_hight_range)) (not (and (> (`KismetMathLibrary.BreakVector2D` _screenlocation) 0.0) (< (`KismetMathLibrary.BreakVector2D` _screenlocation) _returnvalue_x) (> (`.Y` (`KismetMathLibrary.BreakVector2D` _screenlocation)) 0.0) (< (`.Y` (`KismetMathLibrary.BreakVector2D` _screenlocation)) _returnvalue_y))))
                  (set `self.SpawnPoint index` 0)
                  (else
                    (`/Engine/EditorBlueprintResources/StandardMacros.IncrementInt` (`self.SpawnPoint index`)
                      (:`  `
                        (`self.K2_SetActorTransform` (`self.Who to Move to`) (`self.Add to Spawn height` (`SceneComponent.K2_GetComponentToWorld` (`Actor.RootComponent` (`|GetArrayItem` _spawn_points_near_player (`self.SpawnPoint index`))))) false true)))))))
            (:`Is Not Valid`
              (`KismetArrayLibrary.Array_RemoveItem` (`self.Active Zombie array`) (`self.Who to Move to`))
              (set `self.Dont Move` true))))))))

(fn `UserConstructionScript`
  (`parent.UserConstructionScript`)
  (`/Game/HorrorEngine/Blueprints/Core/HorrorEngineMacros.HM_DefaultConstructions` (`self.CreateNewHorrorEvent`))
  (set `self.Tags` (`|MakeArray` (`self.Area / Spawn Point Tag`) (`self.Spawner Tag Identifier`)))
  (`TextRenderComponent.K2_SetText` (`self.TextRender`) (`|FormatText` "Area to Use ({none})" (`KismetTextLibrary.Conv_NameToText` (`|GetArrayItem` (`self.Tags`)))))
  (`TextRenderComponent.K2_SetText` (`self.TextRender1`) (`|FormatText` "Spawnig {none}" (`KismetTextLibrary.Conv_NameToText` (`KismetStringLibrary.Conv_StringToName` (`KismetSystemLibrary.GetClassDisplayName` (`self.WhoToSpawn`))))))
  (switch `/Game/MainLevels/BluePrints/SpawnCollectionToUse` (`self.Spawn Collection to Use`)
    (:`NewEnumerator2`
      (`SceneComponent.SetVisibility` (`self.Plane5`) true true)
      (set `self.Tags` (`|MakeArray` "All Spawn Points" (`self.Spawner Tag Identifier`)))
      (`TextRenderComponent.K2_SetText` (`self.TextRender`) (`KismetTextLibrary.Conv_NameToText` (`|GetArrayItem` (`self.Tags`)))))))