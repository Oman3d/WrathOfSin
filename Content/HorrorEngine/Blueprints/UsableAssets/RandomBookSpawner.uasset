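; RandomBookSpawner relocates an existing Book of Exorcism to a random spawn point when play begins.
; It picks from all RandomSpawns actors, sets the first book's CompatibleActors to SetKeyto, then teleports it to the chosen transform after short delays.
; A HasSpawnedBook flag guards against repeats, and printed warnings report a missing book or missing spawn points.
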(event `self.ReceiveBeginPlay`
  (`self.SpawnBook`))

(event `SpawnBook`
  (if (not (`self.Has Spawned book`))
    (bind _outactors (`GameplayStatics.GetAllActorsOfClass` "/Game/HorrorEngine/Blueprints/UsableAssets/RandomSpawns.RandomSpawns_C"))
    (bind _outitem (`KismetArrayLibrary.Array_Random` _outactors))
    (`/Engine/EditorBlueprintResources/StandardMacros.IsValid` _outitem
      (:`Is Valid`
        (`KismetSystemLibrary.Delay` 0.25)
        (bind _outactors_2 (`GameplayStatics.GetAllActorsOfClass` "/Game/HorrorEngine/Blueprints/UsableAssets/Inventory/BookofExorcismm.BookofExorcismm_C"))
        (bind _output (`|GetArrayItem` _outactors_2))
        (`/Engine/EditorBlueprintResources/StandardMacros.IsValid` _output
          (:`Is Valid`
            (set `/Game/HorrorEngine/Blueprints/UsableAssets/Inventory/Key.CompatibleActors` (`|MakeArray` (`self.SetKeyto`) :!type "/Game/HorrorEngine/Blueprints/Core/Use Object Reference") _output)
            (`KismetSystemLibrary.Delay` 1.0)
            (bind (_sweephitresult _returnvalue) (`self.K2_SetActorTransform` _output (`self.GetTransform` _outitem) false true))
            (set `self.Has Spawned book` _returnvalue))
          (:`Is Not Valid`
            (`KismetSystemLibrary.PrintString` "Add book of Excrcism to world"))))
      (:`Is Not Valid`
        (`KismetSystemLibrary.PrintString` "Add book Spawn points to World")))))

(fn `UserConstructionScript`)