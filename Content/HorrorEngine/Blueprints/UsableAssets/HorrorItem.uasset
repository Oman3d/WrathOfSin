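; HorrorItem is a usable pickup that frightens the player when used.
; On BeginPlay it applies its static mesh with one of five MeshSettings entries chosen at random.
; Use triggers a Horror Engine fear effect with a custom baby sound on the player character, adds to that character's fear, then destroys the item.
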(event `self.ReceiveBeginPlay`
  (`/Game/HorrorEngine/Blueprints/Core/HorrorEngineFunctions.SetMesh` (`self.StaticMesh`) (`|GetArrayItem` (`self.Mesh Settings`) (`KismetMathLibrary.RandomInteger` 5))))

(event `self.Use`
  (params (HorrorEvent :type Boolean))
  (bind _asbp_character_base (cast `/Game/MainLevels/Player/BP_CharacterBase` (`GameplayStatics.GetPlayerCharacter` 0)))
  (`/Game/HorrorEngine/HorrorEngine.Fear` (`/Game/MainLevels/Player/BP_CharacterBase.Horror Engine Ref` _asbp_character_base) (make `/Game/HorrorEngine/Blueprints/Structures/HorrorEvent/HE_Fear` true true "/Game/HorrorEngine/Audio/SFX/Baby01.Baby01"))
  (`/Game/MainLevels/Player/BP_CharacterBase.Add Fear` _asbp_character_base 10.0)
  (`self.K2_DestroyActor`))

(fn `UserConstructionScript`
  (`parent.UserConstructionScript`))