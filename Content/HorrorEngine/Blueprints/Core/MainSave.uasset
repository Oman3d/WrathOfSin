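; MainSave is the save-game object that stores quest progress for the quest manager.
; It holds active, pending and completed quest lists, quest givers, condition tags, the last active quest and new-game state.
; Per-quest records are looked up by unique name, added only once with first-sequence objectives, and replaced in place on update.
; Saving writes itself to its slot, notifies QuestManager on success and prints the result.
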(fn `Add_To_Saved_Quests`
  (params (Quest :type "/Game/QuestManager/Blueprints/Data/Structs/Struct_QuestMaster Structure"))
  (bind ((`UniqueName_59_0187024B451DEEE8C06697B570C8DE65` _uniquename) (`Essentials_83_7D99065F4699AA9B725325B2BD50ECE0` _essentials) (`QuestLogWidget_74_E3A24C404949192A92900B9ED551A80E` _questlogwidget) (`QuestCompletedWidget_71_1F2F748443CB18B47AF067A77CCA33D1` _questcompletedwidget) (`QuestFailedWidget_73_2F8AC4494D592BA908A25581CC8B58D7` _questfailedwidget) (`Sequences_32_428362594EA183BC1B9D879AD2C9242B` _sequences)) (break `/Game/QuestManager/Blueprints/Data/Structs/Struct_QuestMaster` (`local.Quest`)))
  (if (not (`self.Find_In_Saved_Quests` _uniquename))
    (`KismetArrayLibrary.Array_Add` (`self.SavedQuests`) (make `/Game/QuestManager/Blueprints/Data/Structs/SaveGame/Struct_SavedQuest` false _uniquename 0 (`.Objectives_10_7586C19746D93B946BDEF79900896FE8` (break `/Game/QuestManager/Blueprints/Data/Structs/Struct_SequenceMaster` (`|GetArrayItem` _sequences)))))))

(fn `DoesHaveSavedGame`
  (returns (ReturnValue :type Boolean))
  (return (not (`self.NewGame`))))

(fn `Find_In_Saved_Quests`
  (params (QuestUniqueName :type Name))
  (returns (Success :type Boolean) (ReturnValue :type "/Game/QuestManager/Blueprints/Data/Structs/SaveGame/Struct_SavedQuest Structure"))
  (locals (LocReturn :type "/Game/QuestManager/Blueprints/Data/Structs/SaveGame/Struct_SavedQuest Structure") (LocSuccess :type Boolean :default false))
  (for _array_element (`self.SavedQuests`)
    (if (== (`.QuestUniqueName_2_A139EC29465F54A911178CA416DDC038` (break `/Game/QuestManager/Blueprints/Data/Structs/SaveGame/Struct_SavedQuest` _array_element)) (`local.QuestUniqueName`))
      (set `local.LocReturn` _array_element)
      (set `local.LocSuccess` true)
      (break)))
  (return (`local.LocSuccess`) (`local.LocReturn`)))

(fn `HasAnyQuestSaved`
  (returns (ReturnValue :type Boolean))
  (return (!= (`self.LastActiveQuest`) "None")))

(fn `Save_QuestManager`
  (returns (ReturnValue :type Boolean))
  (bind _returnvalue (`GameplayStatics.SaveGameToSlot` self (`self.SaveSlotName`)))
  (if _returnvalue
    (`/Game/QuestManager/Blueprints/Components/Manager_Mission.OnQuestManagerSaved` (`self.QuestManager`))
    (`KismetSystemLibrary.PrintString` null "Quest saved")
    (return true)
    (else
      (`KismetSystemLibrary.PrintString` null "No save")
      (return false))))

(fn `Update_Active_Quest`
  (params (ActiveQuest :type Name) (InQuest :type Boolean))
  (set `self.LastActiveQuest` (`local.ActiveQuest`))
  (set `self.QuestWasActive` (`local.InQuest`)))

(fn `Update_QuestList`
  (params (ActiveQuests :type "Array of /Game/QuestManager/Blueprints/Data/Structs/Struct_QuestMaster Structure") (PendingQuests :type "Array of /Game/QuestManager/Blueprints/Data/Structs/Struct_QuestMaster Structure") (CompletedQuests :type "Array of /Game/QuestManager/Blueprints/Data/Structs/Struct_QuestMaster Structure") (ActiveQuestGivers :type "Array of /Game/QuestManager/Blueprints/Data/Structs/Struct_ActiveQuestGiver Structure") (ConditionTags :type "Array of Name"))
  (set `self.ActiveQuests` ActiveQuests)
  (set `self.PendingQuests` PendingQuests)
  (set `self.CompletedQuests` CompletedQuests)
  (set `self.ActiveQuestGivers` ActiveQuestGivers)
  (set `self.ConditionTags` ConditionTags))

(fn `Update_Saved_Quest`
  (params (NewInfo :type "/Game/QuestManager/Blueprints/Data/Structs/SaveGame/Struct_SavedQuest Structure (by ref)") (QuestUniqueName :type Name))
  (locals (LocIndex :type Integer :default 0))
  (set `local.LocIndex` (`KismetArrayLibrary.Array_Find` (`self.SavedQuests`) (`.ReturnValue` (`self.Find_In_Saved_Quests` QuestUniqueName))))
  (`KismetArrayLibrary.Array_Set` (`self.SavedQuests`) (`local.LocIndex`) (`local.NewInfo`)))