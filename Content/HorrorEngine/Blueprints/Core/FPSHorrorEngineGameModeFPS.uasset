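; Game mode Blueprint for the Horror Engine FPS setup, with an empty BeginPlay and construction script, so it runs no logic of its own.
; A disconnected branch in the event graph checks the level name to create either the main HUD or, on MenuLevel, the main menu with a visible cursor.
; That UI setup never executes.
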(event `self.ReceiveBeginPlay`)

(fn `UserConstructionScript`)