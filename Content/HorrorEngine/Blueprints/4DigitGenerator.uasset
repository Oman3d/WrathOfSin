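; 4DigitGenerator is a helper that generates a random numeric code with a given number of digits.
; GenerateCode builds the number as a string, appending one random digit per loop iteration, then converts it to an integer.
; The first digit is never zero, so the result always keeps the requested length.
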(fn `Generate Code`
  (params (Digits :type Integer))
  (returns (ReturnValue :type Integer))
  (locals (`Generated Number` :type String))
  (for _index (range 1 (+ Digits 1))
    (set `local.Generated Number` (`KismetStringLibrary.Concat_StrStr` (`local.Generated Number`) (`KismetStringLibrary.Conv_IntToString` (select `bool` (== _index 1) :`false` (`KismetMathLibrary.RandomIntegerInRange` 0 9) :`true` (`KismetMathLibrary.RandomIntegerInRange` 1 9))))))
  (return (`KismetStringLibrary.Conv_StringToInt` (`local.Generated Number`))))