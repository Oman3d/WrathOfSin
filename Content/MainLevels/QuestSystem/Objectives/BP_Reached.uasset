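; BP_Reached is a quest objective for reaching a destination actor.
; On activation it calls the parent logic and binds to the destination's begin-overlap event.
; An overlap by a BP_CharacterBase or PossessedPlayer only unbinds that event, as the OnCompleted call is left unconnected.
; GetIsComplete always returns false, so the objective never reports completion itself.
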(event `self.Activate Objective`
  (`parent.Activate Objective`)
  (add `Actor.OnActorBeginOverlap` (`self.Destication`) (delegate `OnActorBeginOverlap_Event_0`)))

(event `OnActorBeginOverlap_Event_0`
  (params (OverlappedActor :type "Actor Object Reference") (OtherActor :type "Actor Object Reference"))
  (cast `/Game/MainLevels/Player/BP_CharacterBase` OtherActor
    (:`then`
      _)
    (:`CastFailed`
      (cast `/Game/MainLevels/Player/PossessedPlayer` OtherActor)))
  (remove `Actor.OnActorBeginOverlap` (`self.Destication`) (delegate `OnActorBeginOverlap_Event_0`)))

(fn `Get Is Complete`
  (returns (`Is Complete` :type Boolean))
  (return false))