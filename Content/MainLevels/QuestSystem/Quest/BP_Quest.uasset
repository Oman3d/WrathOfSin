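; BP_Quest is the base quest actor, holding a root objective collection that child quests build.
; On BeginPlay it constructs that collection, populates its sub-objectives and activates it, with both build functions printing errors unless overridden.
; The construction script shows the root objective's name on a text render.
; Save and load events call SaveVars and LoadVars, which only print placeholder messages here.
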(event `self.ReceiveBeginPlay`
  (bind _root_objcolection (`self.ConstructMainObjectiveCollection`))
  (bind _output_get (set `self.RootObjectiveCollection` _root_objcolection))
  (`self.Populate Sub Objectives` _output_get)
  (`/Game/MainLevels/QuestSystem/Objectives/BP_Objective.Activate Objective` (`self.RootObjectiveCollection`)))

(event `Load_1_1`
  (`self.LoadVars`))

(event `Save_1_1`
  (`self.SaveVars`))

(fn `ConstructMainObjectiveCollection`
  (returns (`Root OBJColection` :type "/Game/MainLevels/QuestSystem/Objectives/BP_OBJColletion Object Reference"))
  (`KismetSystemLibrary.PrintString` "Error: Create Root OBJ Collection Called Base Class!" true true (struct :`R` 1.0 :`A` 1.0))
  (return null))

(fn `Get Root Objective Collection`
  (returns (RootObjectiveCollection :type "/Game/MainLevels/QuestSystem/Objectives/BP_OBJColletion Object Reference"))
  (return (`self.RootObjectiveCollection`)))

(fn `Load`
  (return))

(fn `LoadVars`
  (`KismetSystemLibrary.PrintString` "Load Vars"))

(fn `Populate Sub Objectives`
  (params (`Root OBJCollection` :type "/Game/MainLevels/QuestSystem/Objectives/BP_OBJColletion Object Reference"))
  (`KismetSystemLibrary.PrintString` "Error: Populate Objectives Called Base Class!" true true (struct :`R` 1.0 :`A` 1.0)))

(fn `Save`
  (return))

(fn `SaveVars`
  (`KismetSystemLibrary.PrintString` "Saved Vars"))

(fn `UserConstructionScript`
  (`TextRenderComponent.K2_SetText` (`self.TextRender`) (`/Game/MainLevels/QuestSystem/Objectives/BP_Objective.Get Objective Name` (`self.RootObjectiveCollection`))))