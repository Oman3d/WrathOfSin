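; Team-specific player spawn point Blueprint that carries a team assignment and can be briefly disabled after use.
; The construction script copies its TEAM value into the BPCTeam component and sets a text render label to match the team, including a Hostile option.
; JustBeenUsed marks the point invalid, then restores it after a short delay so it is temporarily unavailable for spawning.
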(event `JustBeenUsed`
  (set `self.PointIsValid` false)
  (`KismetSystemLibrary.Delay` 3.0)
  (set `self.PointIsValid` true))

(fn `UserConstructionScript`
  (bind _bpc_team (`self.BPC_Team`))
  (set `/Game/BSP_DABB/Blueprints/Components/BPC_Team.BSP_Team` (`self.TEAM`) _bpc_team)
  (switch `/Game/BSP_DABB/Enumerator/E_TeamList` (`/Game/BSP_DABB/Blueprints/Components/BPC_Team.BSP_Team` _bpc_team)
    (:`NewEnumerator0`
      (`TextRenderComponent.K2_SetText` (`self.TextRender`) (`self.Team1`)))
    (:`NewEnumerator1`
      (`TextRenderComponent.K2_SetText` (`self.TextRender`) (`self.Team2`)))
    (:`NewEnumerator2`
      (`TextRenderComponent.K2_SetText` (`self.TextRender`) (`self.Team3`)))
    (:`NewEnumerator3`
      (`TextRenderComponent.K2_SetText` (`self.TextRender`) (`self.Team4`)))
    (:`NewEnumerator4`
      (`TextRenderComponent.K2_SetText` (`self.TextRender`) (`self.HOSSTILE`)))))