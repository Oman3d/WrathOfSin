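; Behavior Tree service for the zombie AI that finds a visible enemy target when a search starts.
; A sphere overlap around the zombie gathers bone-break characters, filtering out teammates and the dead through their team component.
; It keeps the previous target if still eligible, otherwise takes the first candidate.
; A line trace must hit that target before its actor and location are written to the Blackboard.
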(event `self.ReceiveSearchStart`
  (params (OwnerActor :type "Actor Object Reference"))
  (bind _bsp_zombie_actorinvisabilitysphere (`self.BSP_Zombie_ActorInVisabilitySphere`))
  ;[0.5569 0.5569 0.5569] Check AI Consinsus for AI location
  (`/Engine/EditorBlueprintResources/StandardMacros.IsValid` OwnerActor
    (:`Is Valid`
      (bind _asbp_ai_zombie_controller (cast `/Game/BSP_DABB/Blueprints/AI_Controller/Zombie/BP_AI_Zombie_Controller` OwnerActor))
      (`/Engine/EditorBlueprintResources/StandardMacros.IsValid` _asbp_ai_zombie_controller
        (:`Is Valid`
          ;;[0.07451 0.1216 0.2706] Task
          (set `self.BSP_Zombie_AIControllerRef` _asbp_ai_zombie_controller)
          (bind _returnvalue (`Actor.K2_GetActorLocation` (`Controller.K2_GetPawn` _asbp_ai_zombie_controller)))
          (set `self.BSP_Zombie_CurrentLocation` _returnvalue)
          ;[0.07451 0.1216 0.2706] Trace For Visabity in colission Shpere
          (bind (_outactors _returnvalue_2) (`KismetSystemLibrary.SphereOverlapActors` _returnvalue 1000.0 (`self.BSP_Zombie_DesiredTargetTypes`) "/Game/BSP_DABB/Blueprints/Characters/PlayerCharacter/BP_BoneBreak_Character.BP_BoneBreak_Character_C" (`|MakeArray` (`Controller.K2_GetPawn` (`self.BSP_Zombie_AIControllerRef`)) :!type "Actor Object Reference")))
          (if _returnvalue_2
            (set `self.BSP_Zombie_KeepCurentTarget` false)
            (`KismetArrayLibrary.Array_Clear` (`self.BSP_Zombie_ActorsCurrentlyInSphere`))
            (for _array_element _outactors
              ;[0.2705 0.2705 0.2705] Process Container
              (`/Engine/EditorBlueprintResources/StandardMacros.IsValid` _array_element
                (:`Is Valid`
                  (bind _ignore (`self.BSP_ActorInSameTeam` _array_element))
                  (if (not _ignore)
                    (bind _returnvalue_3 (`Actor.GetComponentByClass` _array_element "/Game/BSP_DABB/Blueprints/Components/BPC_Team.BPC_Team_C"))
                    ;;[1 1 1] check if dead
                    (`/Engine/EditorBlueprintResources/StandardMacros.IsValid` _returnvalue_3
                      (:`Is Valid`
                        (if (`/Game/BSP_DABB/Blueprints/Components/BPC_Team.IsDead` _returnvalue_3)
                          _
                          (elif (and (== _array_element _bsp_zombie_actorinvisabilitysphere) (`KismetSystemLibrary.IsValid` _bsp_zombie_actorinvisabilitysphere))
                            (set `self.BSP_Zombie_KeepCurentTarget` true)
                            (else
                              (`KismetArrayLibrary.Array_AddUnique` (`self.BSP_Zombie_ActorsCurrentlyInSphere`) _array_element))))))))))
            ;[0.07451 0.1216 0.2706] Trace For Visabity in colission Shpere
            (if (`self.BSP_Zombie_KeepCurentTarget`)
              (`/Engine/EditorBlueprintResources/StandardMacros.IsValid` (`self.BSP_Zombie_ActorInVisabilitySphere`)
                (:`Is Valid`
                  ;[0.07451 0.1216 0.2706] Second check to confirm target is visable and in range
                  (bind _outhit (`KismetSystemLibrary.LineTraceSingle` (`self.BSP_Zombie_CurrentLocation`) (`Actor.K2_GetActorLocation` (`self.BSP_Zombie_ActorInVisabilitySphere`)) "TraceTypeQuery3" true (`|MakeArray` (`Controller.K2_GetPawn` (`self.BSP_Zombie_AIControllerRef`)) :!type "Actor Object Reference") :!label _label))
                  ;[0.07451 0.1216 0.2706] Update
                  ;;[1 1 1] No Idea Why this has to be false but for some reason its the only way it works
                  (if (== (`.HitActor` (`GameplayStatics.BreakHitResult` _outhit)) (`self.BSP_Zombie_ActorInVisabilitySphere`))
                    ;;[1 1 1] Set BlackBoard
                    (`BTFunctionLibrary.SetBlackboardValueAsObject` (`self.BSP_Zombie_AITarget`) (`self.BSP_Zombie_ActorInVisabilitySphere`))
                    (`BTFunctionLibrary.SetBlackboardValueAsVector` (`self.BSP_Zombie_TargetLocation`) (`Actor.K2_GetActorLocation` (`self.BSP_Zombie_ActorInVisabilitySphere`)))))
                (:`Is Not Valid`
                  (set `self.BSP_Zombie_AITarget` (struct))
                  (set `self.BSP_Zombie_TargetLocation` (struct))))
              (else
                (for (_array_element_2 _array_index) (`self.BSP_Zombie_ActorsCurrentlyInSphere`)
                  (`/Engine/EditorBlueprintResources/StandardMacros.IsValid` _array_element_2
                    (:`Is Valid`
                      (if (== _array_index 0)
                        (set `self.BSP_Zombie_ActorInVisabilitySphere` _array_element_2)))))
                (`/Engine/EditorBlueprintResources/StandardMacros.IsValid` (`self.BSP_Zombie_ActorInVisabilitySphere`)
                  (:`Is Valid`
                    (goto _label)))))))))))

(fn `BSP_ActorInSameTeam`
  (params (InputPin :type "Actor Object Reference"))
  (returns (Ignore :type Boolean))
  (bind (_resultinvalid _bsp_team) (`self.BSP_GetOwnerTeam`))
  (bind _returnvalue (`Actor.GetComponentByClass` InputPin "/Game/BSP_DABB/Blueprints/Components/BPC_Team.BPC_Team_C"))
  (`/Engine/EditorBlueprintResources/StandardMacros.IsValid` InputPin
    (:`Is Valid`
      (if _resultinvalid
        (return true)
        (else
          (`/Engine/EditorBlueprintResources/StandardMacros.IsValid` _returnvalue
            (:`Is Valid`
              (if (`|EnumEquality` _bsp_team (`/Game/BSP_DABB/Blueprints/Components/BPC_Team.BSP_Team` _returnvalue))
                (return true)
                (else
                  _)))
            (:`Is Not Valid`
              _))
          (return false))))
    (:`Is Not Valid`
      (return true))))

(fn `BSP_GetOwnerTeam`
  (returns (ResultInvalid :type Boolean) (BSP_Team :type "/Game/BSP_DABB/Enumerator/E_TeamList Enum"))
  (bind _returnvalue (`Actor.GetComponentByClass` (`Controller.K2_GetPawn` (`self.BSP_Zombie_AIControllerRef`)) "/Game/BSP_DABB/Blueprints/Components/BPC_Team.BPC_Team_C"))
  (`/Engine/EditorBlueprintResources/StandardMacros.IsValid` _returnvalue
    (:`Is Valid`
      (return false (`/Game/BSP_DABB/Blueprints/Components/BPC_Team.BSP_Team` _returnvalue)))
    (:`Is Not Valid`
      (return true "NewEnumerator4"))))