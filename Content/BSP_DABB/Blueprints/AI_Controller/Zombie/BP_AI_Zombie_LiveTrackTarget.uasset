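; Behavior tree task that updates a zombie's target location to track the player.
; It casts the controlled pawn to BP_Zombie and branches on its Intelligence: Stoopid fails the task immediately.
; Little Smarter writes player character 0's current location to the target location Blackboard key and succeeds.
; A failed cast or invalid player leaves the task without a FinishExecute call.
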(event `self.ReceiveExecuteAI`
  (params (OwnerController :type "AIController Object Reference") (ControlledPawn :type "Pawn Object Reference"))
  (bind _returnvalue (`GameplayStatics.GetPlayerCharacter` 0))
  ;[0.07451 0.1216 0.2706] Live track AI
  (bind _asbp_zombie (cast `/Game/BSP_DABB/Blueprints/Characters/AI/Zombie/BP_Zombie` ControlledPawn))
  (switch `/Game/BSP_DABB/Enumerator/E_HowStoopid` (`/Game/BSP_DABB/Blueprints/Characters/AI/Zombie/BP_Zombie.Intelligence` _asbp_zombie)
    (:`NewEnumerator0`
      (`self.FinishExecute` false))
    (:`NewEnumerator4`
      (`/Engine/EditorBlueprintResources/StandardMacros.IsValid` _returnvalue
        (:`Is Valid`
          (`BTFunctionLibrary.SetBlackboardValueAsVector` (`self.BSP_Zombie_TargetLocation`) (`Actor.K2_GetActorLocation` _returnvalue))
          (`self.FinishExecute` true))))))

(fn `OnRep_BSP_Zombie_TargetLocation`)