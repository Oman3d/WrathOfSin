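; Weapon container component that tracks a character's primary and active weapons and keeps the matching animation set applied.
; When the active weapon replicates, its RepNotify flags it in use and copies that weapon's animations into the instigator's BoneData component, falling back to the unarmed set.
; A force-unarm event forwards to the owning BoneBreak character.
; Socket getters return attach sockets, though the secondary getter also reads the primary weapon.
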(event `DABB_ForceUnarmed`
  (bind _asbp_bone_break_character (cast `/Game/BSP_DABB/Blueprints/Characters/PlayerCharacter/BP_BoneBreak_Character` (`self.GetOwner`)))
  (`/Game/BSP_DABB/Blueprints/Characters/PlayerCharacter/BP_BoneBreak_Character.CallForceUnarm` _asbp_bone_break_character))

(fn `f_DABB_Get_OwningWeaponActive_Component`
  (returns (Owning_WeaponActive :type "/Game/BSP_DABB/Blueprints/Weapons/BP_Weapon_Master Object Reference") (WeaponBoneComponentRef :type "/Game/BSP_DABB/Blueprints/Components/BPC_DABB_WeaponData Object Reference"))
  (bind _owning_weaponactive (`self.Owning_WeaponActive`))
  (`/Engine/EditorBlueprintResources/StandardMacros.IsValid` _owning_weaponactive
    (:`Is Valid`
      (return (`self.Owning_WeaponActive`) (`/Game/BSP_DABB/Blueprints/Weapons/BP_Weapon_Master.BPC_DABB_WeaponData` _owning_weaponactive)))
    (:`Is Not Valid`
      (return null null))))

(fn `f_DABB_GetPrimarySocket`
  (returns (Item :type Name))
  (bind _weapon_primary (`self.Weapon_Primary`))
  (`/Engine/EditorBlueprintResources/StandardMacros.IsValid` _weapon_primary
    (:`Is Valid`
      (return (`Actor.GetAttachParentSocketName` _weapon_primary)))
    (:`Is Not Valid`
      (return "None"))))

(fn `f_DABB_GetSecondarySocket`
  (returns (Item :type Name))
  (bind _weapon_primary (`self.Weapon_Primary`))
  (`/Engine/EditorBlueprintResources/StandardMacros.IsValid` _weapon_primary
    (:`Is Valid`
      (return (`Actor.GetAttachParentSocketName` _weapon_primary)))
    (:`Is Not Valid`
      (return "None"))))

(fn `OnRep_Owning_WeaponActive`
  (bind (_owning_weaponactive _weaponbonecomponentref) (`self.f_DABB_Get_OwningWeaponActive_Component`))
  (bind (_owning_weaponactive_2 _weaponbonecomponentref_2) (`self.f_DABB_Get_OwningWeaponActive_Component`))
  (bind (_owning_weaponactive_3 _weaponbonecomponentref_3) (`self.f_DABB_Get_OwningWeaponActive_Component`))
  (bind _owning_weaponactive_4 (`self.Owning_WeaponActive`))
  (bind _returnvalue (`Actor.GetComponentByClass` (`Actor.Instigator` (`self.GetOwner`)) "/Game/BSP_DABB/Blueprints/Components/BPC_DABB_BoneData.BPC_DABB_BoneData_C"))
  (bind _returnvalue_2 (`Actor.GetComponentByClass` (`Actor.Instigator` (`self.GetOwner`)) "/Game/BSP_DABB/Blueprints/Components/BPC_DABB_BoneData.BPC_DABB_BoneData_C"))
  (`|ExecutionSequence`
    (:`then_0`
      ;[0.302 0.3647 0.5216] Send the set active weapon to the AnimInstance
      (`/Engine/EditorBlueprintResources/StandardMacros.IsValid` _owning_weaponactive_4
        (:`Is Valid`
          (`/Game/BSP_DABB/Blueprints/Weapons/BP_Weapon_Master.Set Weapon Inuse` _owning_weaponactive_4 true))
        (:`Is Not Valid`
          _))
      (`/Engine/EditorBlueprintResources/StandardMacros.IsValid` _weaponbonecomponentref
        (:`Is Valid`
          (bind _st_owning_charater_weapon_animation_state (`/Game/BSP_DABB/Blueprints/Components/BPC_DABB_WeaponData.f_DABB_Get_Weapon_Animations` _weaponbonecomponentref))
          (`/Engine/EditorBlueprintResources/StandardMacros.IsValid` _owning_weaponactive
            (:`Is Valid`
              (set `/Game/BSP_DABB/Blueprints/Components/BPC_DABB_BoneData.ST_CurrentWeaponAnimations` _st_owning_charater_weapon_animation_state _returnvalue))
            (:`Is Not Valid`
              (set `/Game/BSP_DABB/Blueprints/Components/BPC_DABB_BoneData.ST_CurrentWeaponAnimations` (`self.Null`) _returnvalue :!label _label))))
        (:`Is Not Valid`
          (goto _label))))
    (:`then_1`
      ;[1 1 1] Reset the Previous animation set
      (`/Engine/EditorBlueprintResources/StandardMacros.IsValid` _owning_weaponactive_2
        (:`Is Valid`
          (bind _st_owning_charater_weapon_animation_state_2 (`/Game/BSP_DABB/Blueprints/Components/BPC_DABB_WeaponData.f_DABB_Get_Weapon_Animations` _weaponbonecomponentref_2))
          (set `/Game/BSP_DABB/Blueprints/Components/BPC_DABB_BoneData.ST_CurrentWeaponAnimations` _st_owning_charater_weapon_animation_state_2 (`Actor.GetComponentByClass` (`Actor.Instigator` (`self.GetOwner`)) "/Game/BSP_DABB/Blueprints/Components/BPC_DABB_BoneData.BPC_DABB_BoneData_C")))))
    (:`then_2`
      ;[1 1 1] Reset Current Animation Set for weapon
      (`/Engine/EditorBlueprintResources/StandardMacros.IsValid` _owning_weaponactive_3
        (:`Is Valid`
          (bind _st_owning_charater_weapon_animation_state_3 (`/Game/BSP_DABB/Blueprints/Components/BPC_DABB_WeaponData.f_DABB_Get_Weapon_Animations` _weaponbonecomponentref_3))
          (set `/Game/BSP_DABB/Blueprints/Components/BPC_DABB_BoneData.ST_CurrentWeaponAnimations` _st_owning_charater_weapon_animation_state_3 (`Actor.GetComponentByClass` (`Actor.Instigator` (`self.GetOwner`)) "/Game/BSP_DABB/Blueprints/Components/BPC_DABB_BoneData.BPC_DABB_BoneData_C")))
        (:`Is Not Valid`
          (set `/Game/BSP_DABB/Blueprints/Components/BPC_DABB_BoneData.ST_CurrentWeaponAnimations` (`/Game/BSP_DABB/Blueprints/Components/BPC_DABB_BoneData.ST_Unarmed` _returnvalue_2) _returnvalue_2))))
    (:`then_3`
      (return))))