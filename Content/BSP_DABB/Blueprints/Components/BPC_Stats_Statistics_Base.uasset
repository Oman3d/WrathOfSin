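; Base stat component that holds one value, starts it at StartingValue and raises or lowers it, as a parent for specific stats.
; Looping timers apply AffectorValue at LoopsPerSecond for gradual change, while separate functions apply one-off amounts.
; Reaching Minimum or Maximum either sets Dead, if flagged, or stops gradual change; values are not clamped.
; Changes within limits call FProcessStepCheck, an empty hook here.
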(event `self.ReceiveBeginPlay`
  ;[0.2706 0.2706 0.2706] Set Starting Value as Current Value
  (set `self.CurrentValue` (`self.StartingValue`)))

(event `IR_Replicated_Incremental_Increase_Start`
  ;[0.2706 0.2706 0.2706] Set Timer for function name incremental increase
  (bind _returnvalue (`KismetSystemLibrary.K2_SetTimer` null "IR_Process_Stats_Incremental_Increase" (`self.f_Process_LoopPerSecond`) true))
  (set `self.ActiveTimerIncrease` _returnvalue))

(event `IR_Replicated_Incremental_Increase_Stop`
  ;[0.2706 0.2706 0.2706] Set Timer for function name incremental increase
  (if (`KismetSystemLibrary.K2_IsValidTimerHandle` (`self.ActiveTimerIncrease`))
    (`KismetSystemLibrary.K2_ClearAndInvalidateTimerHandle` (`self.ActiveTimerIncrease`))))

(event `IR_Replicated_Incremental_Decrease_Start`
  ;[0.2706 0.2706 0.2706] Set Timer for function name incremental Decrease
  (bind _returnvalue (`KismetSystemLibrary.K2_SetTimer` null "IR_Process_Stats_Incremental_Decrease" (`self.f_Process_LoopPerSecond`) true))
  (set `self.ActiveTimerDecrease` _returnvalue))

(event `IR_Replicated_Incremental_Decrease_Stop`
  ;[0.2706 0.2706 0.2706] Set Timer for function name incremental Decrease
  (if (`KismetSystemLibrary.K2_IsValidTimerHandle` (`self.ActiveTimerDecrease`))
    (`KismetSystemLibrary.K2_ClearAndInvalidateTimerHandle` (`self.ActiveTimerDecrease`))))

(fn `f_Process_LoopPerSecond`
  (returns (ReturnValue :type "Float (double-precision)"))
  (return (/ 1.0 (`self.LoopsPerSecond`))))

(fn `f_Process_SetValues`
  (params (AffectorValue :type "Float (double-precision)") (LoopsPerSecond :type "Float (double-precision)"))
  (set `self.AffectorValue` AffectorValue)
  (set `self.LoopsPerSecond` LoopsPerSecond)
  (return))

(fn `f_Process_StepCheck`)

(fn `IR Process Stats Increase`
  (params (IncreaseValue :type "Float (double-precision)"))
  ;[0.2706 0.2706 0.2706] Incrementally increase the value of the component
  ;;[0.07451 0.1216 0.2706] Check value is not more than maximum and set incremental steps
  (if (>= (`self.CurrentValue`) (`self.Maximum`))
    ;;[0.07451 0.1216 0.2706] If limit is reached cause death.
    (if (`self.bIf_Maximum_Cause_Death`)
      (set `self.bDead` true)
      (return)
      (else
        (return)))
    (else
      (set `self.CurrentValue` (+ (`self.CurrentValue`) (`local.IncreaseValue`)))
      (`self.f_Process_StepCheck`)
      (return))))

(fn `IR_Process_Stats_Decrease`
  (params (DecreaseValue :type "Float (double-precision)"))
  ;[0.2706 0.2706 0.2706] Incrementally increase the value of the component
  ;;[0.07451 0.1216 0.2706] Check value is not more than maximum and set incremental steps
  (set `self.CurrentValue` (- (`self.CurrentValue`) (`local.DecreaseValue`)))
  (if (<= (`self.CurrentValue`) (`self.Minimum`))
    ;;[0.07451 0.1216 0.2706] If limit is reached cause death.
    (if (`self.bIf_Minimum_Cause_Death`)
      (set `self.bDead` true)
      (return)
      (else
        (return)))
    (else
      (`self.f_Process_StepCheck`)
      (return))))

(fn `IR_Process_Stats_Incremental_Decrease`
  ;[0.2706 0.2706 0.2706] Incrementally increase the value of the component
  ;;[0.07451 0.1216 0.2706] Check value is not more than maximum and set incremental steps
  (if (<= (`self.CurrentValue`) (`self.Minimum`))
    ;;[0.07451 0.1216 0.2706] If limit is reached cause death.
    (if (`self.bIf_Minimum_Cause_Death`)
      (set `self.bDead` true)
      (return)
      (else
        (`self.IR_Replicated_Incremental_Decrease_Stop`)
        (return)))
    (else
      (set `self.CurrentValue` (- (`self.CurrentValue`) (`self.AffectorValue`)))
      (`self.f_Process_StepCheck`)
      (return))))

(fn `IR_Process_Stats_Incremental_Increase`
  ;[0.2706 0.2706 0.2706] Incrementally increase the value of the component
  ;;[0.07451 0.1216 0.2706] Check value is not more than maximum and set incremental steps
  (if (>= (`self.CurrentValue`) (`self.Maximum`))
    ;;[0.07451 0.1216 0.2706] If limit is reached cause death.
    (if (`self.bIf_Maximum_Cause_Death`)
      (set `self.bDead` true)
      (return)
      (else
        (`self.IR_Replicated_Incremental_Increase_Stop`)
        (return)))
    (else
      (set `self.CurrentValue` (+ (`self.CurrentValue`) (`self.AffectorValue`)))
      (`self.f_Process_StepCheck`)
      (return))))