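; BP_DoorGarage is a garage door actor that reacts to characters entering or leaving its trigger volume.
; On begin and end overlap with a BP_CharacterBase, it sets the PlayerNear flag on the GarageDoor mesh's AnimBP_DoorGarage instance.
; The door's motion is left to that Animation Blueprint, and a debug string is drawn if the anim instance cast fails.
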(event `self.ReceiveBeginPlay`)

(event `self.Trigger.OnComponentBeginOverlap`
  (params (OverlappedComponent :type "PrimitiveComponent Object Reference") (OtherActor :type "Actor Object Reference") (OtherComp :type "PrimitiveComponent Object Reference") (OtherBodyIndex :type Integer) (bFromSweep :type Boolean) (SweepResult :type "HitResult Structure (by ref)"))
  (cast `/Game/FPS_Game/Blueprints/BP_CharacterBase` OtherActor)
  (bind _asanim_bp_door_garage (cast `/Game/HQ_ResidentialHouse/Meshes/DoorGarage/AnimBP_DoorGarage` (`SkeletalMeshComponent.GetAnimInstance` (`self.Garage_door`)))
    (:`then`
      (set `/Game/HQ_ResidentialHouse/Meshes/DoorGarage/AnimBP_DoorGarage.PlayerNear` true _asanim_bp_door_garage))
    (:`CastFailed`
      (`KismetSystemLibrary.DrawDebugString` (0.0 0.0 0.0) "Something wrong" null (struct :`R` 1.0 :`G` 1.0 :`B` 1.0 :`A` 1.0) 4.0 :!label _label))))

(event `self.Trigger.OnComponentEndOverlap`
  (params (OverlappedComponent :type "PrimitiveComponent Object Reference") (OtherActor :type "Actor Object Reference") (OtherComp :type "PrimitiveComponent Object Reference") (OtherBodyIndex :type Integer))
  (cast `/Game/FPS_Game/Blueprints/BP_CharacterBase` OtherActor)
  (bind _asanim_bp_door_garage (cast `/Game/HQ_ResidentialHouse/Meshes/DoorGarage/AnimBP_DoorGarage` (`SkeletalMeshComponent.GetAnimInstance` (`self.Garage_door`)))
    (:`then`
      (set `/Game/HQ_ResidentialHouse/Meshes/DoorGarage/AnimBP_DoorGarage.PlayerNear` false _asanim_bp_door_garage))
    (:`CastFailed`
      (goto _label))))

(fn `UserConstructionScript`)