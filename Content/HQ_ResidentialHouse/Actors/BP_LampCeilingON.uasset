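; BP_LampCeilingON is a ceiling lamp actor for the residential house set, with a switchable on/off state.
; The Construction Script passes LightSettings to SetPointlight, then creates a dynamic material instance on the glass mesh.
; LightOnOff sets both the glass emission intensity and the point light visibility, so glow and lighting match.
; All setup happens at construction; the event graph has no runtime logic.
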(fn `UserConstructionScript`
  (`/Game/HorrorEngine/Blueprints/Core/HorrorEngineFunctions.SetPointlight` null (`self.Light Settings`))
  (bind _returnvalue (`PrimitiveComponent.CreateDynamicMaterialInstance` (`self.LampCeiling_Glass`) 0 "/Game/HQ_ResidentialHouse/Materials/Mat_LampsCeiling.Mat_LampsCeiling" "None"))
  (if (`self.Light On/Off`)
    (`MaterialInstanceDynamic.SetScalarParameterValue` _returnvalue "Emission Intensity" 15.0)
    (`SceneComponent.SetVisibility` (`self.PointLight`) true false)
    (else
      (`MaterialInstanceDynamic.SetScalarParameterValue` _returnvalue "Emission Intensity" 0.0)
      (`SceneComponent.SetVisibility` (`self.PointLight`) false false))))